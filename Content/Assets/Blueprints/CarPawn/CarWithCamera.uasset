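; Player car pawn for an endless two-lane driving game, with speed and timer components, engine audio and a bounce timeline.
; ChangeRoad plays or reverses a swerve timeline to lerp lanes, choosing its curve by speed.
; Front and back hitboxes notify CarTiles, exploding and stopping the game unless it is an obstacle point.
; Tick triggers game over once the explosion emitter expires, while a trigger destroys passed tiles.
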(event OnComponentBeginOverlap(CarHitBoxFront)
  (params (OverlappedComponent :type Primitive%20Component%20Object%20Reference) (OtherActor :type Actor%20Object%20Reference) (OtherComp :type Primitive%20Component%20Object%20Reference) (OtherBodyIndex :type Integer) (bFromSweep :type Boolean) (SweepResult :type Hit%20Result%20Structure%20%28by%20ref%29))
  (bind _returnvalue (Game|GetPlayerController 0))
  (bind _asendless_pc (Utilities|Casting|CastToEndlessPC _returnvalue))
  ;[1 1 1] Collision on obstacle
  (bind _ascar_tile (Utilities|Casting|CastToCarTile OtherActor))
  (if (Components|ComponentHasTag OtherComp "Collision")
    (Default|OnCollisionwithCar _ascar_tile false)
    (if (not (Variables|/Game/Assets/Blueprints/FloorTile/FloorTile.FloorTile_C|GetIsObstaclePoint _ascar_tile))
      (Variables|/Game/Assets/Blueprints/FloorTile/FloorTile.FloorTile_C|SetIsObstaclePoint _ascar_tile false)
      (CallFunction|StartExplosion true)
      (Default|RemoveUI (.AsEndless%20HUD (Utilities|Casting|CastToEndlessHUD (HUD|GetHUD _asendless_pc))) "NewEnumerator0")
      (Default|StopGame _asendless_pc)
      (Audio|Components|Audio|Stop (Variables|Default|GetCarEngine)))))

(event OnComponentBeginOverlap(Trgr_Destroy)
  (params (OverlappedComponent :type Primitive%20Component%20Object%20Reference) (OtherActor :type Actor%20Object%20Reference) (OtherComp :type Primitive%20Component%20Object%20Reference) (OtherBodyIndex :type Integer) (bFromSweep :type Boolean) (SweepResult :type Hit%20Result%20Structure%20%28by%20ref%29))
  ;[1 1 1] Trgr_Destroy component destroys floor tile actors on overlap. Meaning, when the floor tile actor is out of camera
  (CallFunction|DestroyFloorTile OtherActor OtherComp))

(event OnComponentBeginOverlap(CarHitBoxBack)
  (params (OverlappedComponent :type Primitive%20Component%20Object%20Reference) (OtherActor :type Actor%20Object%20Reference) (OtherComp :type Primitive%20Component%20Object%20Reference) (OtherBodyIndex :type Integer) (bFromSweep :type Boolean) (SweepResult :type Hit%20Result%20Structure%20%28by%20ref%29))
  (bind _returnvalue (Game|GetPlayerController 0))
  (bind _asendless_pc (Utilities|Casting|CastToEndlessPC _returnvalue))
  ;[1 1 1] Collision on obstacle
  (bind _ascar_tile (Utilities|Casting|CastToCarTile OtherActor))
  (if (Components|ComponentHasTag OtherComp "Collision")
    (Default|OnCollisionwithCar _ascar_tile true)
    (if (not (Variables|/Game/Assets/Blueprints/FloorTile/FloorTile.FloorTile_C|GetIsObstaclePoint _ascar_tile))
      (Variables|/Game/Assets/Blueprints/FloorTile/FloorTile.FloorTile_C|SetIsObstaclePoint _ascar_tile false)
      (CallFunction|StartExplosion false)
      (Default|RemoveUI (.AsEndless%20HUD (Utilities|Casting|CastToEndlessHUD (HUD|GetHUD _asendless_pc))) "NewEnumerator0")
      (Default|StopGame _asendless_pc)
      (Audio|Components|Audio|Stop (Variables|Default|GetCarEngine)))))

(event Custom|ChangeRoad
  ;[1 1 1] Switches Car location from left to right and vice versa
  (if (Variables|Default|GetisOnRightLane)
    (if (Variables|Default|GetCanSwerve)
      (Variables|Default|SetCanSwerve false)
      (bind (_direction _alpha _fasteralpha) (Timeline|Swerve PlayFromStart)
        (:Update
          (if (> (Default|GetSpeed (Variables|Default|GetSpeedManager)) 145.0)
            (CallFunction|UpdateCarLocation _alpha)
            (else
              (CallFunction|UpdateCarLocation _fasteralpha))))
        (:Finished
          (Variables|Default|SetisOnRightLane (not (Variables|Default|GetisOnRightLane)))
          (Variables|Default|SetCanSwerve true))))
    (elif (Variables|Default|GetCanSwerve)
      (Variables|Default|SetCanSwerve false)
      (Timeline|Swerve ReverseFromEnd))))

(event Custom|StopSwerve
  ;[1 1 1] Switches Car location from left to right and vice versa
  (bind (_direction _alpha _fasteralpha) (Timeline|Swerve Stop)
    (:Update
      (if (> (Default|GetSpeed (Variables|Default|GetSpeedManager)) 145.0)
        (CallFunction|UpdateCarLocation _alpha)
        (else
          (CallFunction|UpdateCarLocation _fasteralpha))))
    (:Finished
      (Variables|Default|SetisOnRightLane (not (Variables|Default|GetisOnRightLane)))
      (Variables|Default|SetCanSwerve true))))

(event Custom|ResetDoOnce
  ;[1 1 1] Checks if particle is activated and is finished
  (Utilities|FlowControl|DoOnce false) ; enters at Reset
)

(event Custom|StopBounce
  ;[1 1 1] Makes the Car Bounce
  (bind _scale (Timeline|Bounce_Timeline Stop)
    (:Update
      (Transformation|SetRelativeScale3D (Variables|Default|GetCar) (Math|Vector|MakeVector 1.0 1.0 _scale)))))

(event Custom|StartBounce
  ;[1 1 1] Makes the Car Bounce
  (bind _scale (Timeline|Bounce_Timeline Play)
    (:Update
      (Transformation|SetRelativeScale3D (Variables|Default|GetCar) (Math|Vector|MakeVector 1.0 1.0 _scale)))))

(event Custom|OnExplosionFinished
  ;[1 1 1] Called when explosion particle finished
  (Default|OnGameOver (.AsEndless%20PC (Utilities|Casting|CastToEndlessPC (Game|GetPlayerController 0))))
  (Variables|Default|SetisOnRightLane true))

(event EventBeginPlay
  (bind _carengine (Variables|Default|GetCarEngine))
  (CallFunction|StartBounce)
  (bind _output_get (Variables|/Game/Assets/Blueprints/ActorComponent/SpeedManager.SpeedManager_C|SetPCRef (Variables|Default|GetSpeedManager) (.AsEndless%20PC (Utilities|Casting|CastToEndlessPC (Game|GetPlayerController 0)))))
  (Variables|/Game/Assets/Blueprints/ActorComponent/TimerManager.TimerManager_C|SetPCRef (Variables|Default|GetTimerManager) _output_get)
  (Audio|Components|Audio|SetSound _carengine "/Game/Assets/Audio/Car/SC_CarStart.SC_CarStart")
  (Audio|Components|Audio|Play _carengine 0.0))

(event EventTick
  (params (DeltaSeconds :type Float%20%28single-precision%29))
  ;[1 1 1] Checks if particle is activated and is finished
  (if (Variables|Default|GetParticleActivated)
    (Utilities|IsValid (Variables|Default|GetExplosionParticleRef)
      (:Is%20Not%20Valid
        (Utilities|FlowControl|DoOnce false
          (:Completed
            (CallFunction|OnExplosionFinished)))))))

(fn ConstructionScript
  (Variables|Default|SetInitialCarLocation (Variables|/Script/Engine.SceneComponent|GetRelativeLocation (Variables|Default|GetCar))))

(fn DestroyFloorTile
  (params (ActorOverlapped :type Actor%20Object%20Reference) (ComponentOverlapped :type Primitive%20Component%20Object%20Reference))
  (Utilities|Casting|CastToCarTile ActorOverlapped
    (:then
      (if (Components|ComponentHasTag ComponentOverlapped "TileEnd")
        (Actor|DestroyActor (stale _asfloor_tile) :!label _label)))
    (:CastFailed
      (bind _asfloor_tile (Utilities|Casting|CastToFloorTile ActorOverlapped))
      (goto _label))))

(fn StartCar
  (bind _carengine (Variables|Default|GetCarEngine))
  (Variables|/Game/Assets/Blueprints/ActorComponent/SpeedManager.SpeedManager_C|SetCanMove (Variables|Default|GetSpeedManager) true)
  (CallFunction|StartBounce)
  (Variables|Default|SetParticleActivated false)
  (CallFunction|ResetDoOnce)
  (Audio|Components|Audio|SetSound _carengine "/Game/Assets/Audio/Car/RunningLoop/SC_CarRunning.SC_CarRunning")
  (Audio|Components|Audio|Play _carengine 0.0))

(fn StopCar
  (Variables|/Game/Assets/Blueprints/ActorComponent/SpeedManager.SpeedManager_C|SetCanMove (Variables|Default|GetSpeedManager) false)
  (CallFunction|StopBounce)
  (CallFunction|StopSwerve))

(fn OnRestart
  (CallFunction|RestartCarPosition)
  (Default|Restart (Variables|Default|GetSpeedManager) (Variables|Default|GetInitialSpeed))
  (Default|OnDeactivate (Variables|Default|GetTimerManager)))

(fn StartExplosion
  (params (IsFront :type Boolean))
  (if IsFront
    (bind _returnvalue (Effects|SpawnEmitteratLocation (Variables|Default|GetExplosionParticle) (Transformation|GetWorldLocation (Variables|Default|GetExplosionPointFront))))
    (Variables|Default|SetExplosionParticleRef _returnvalue)
    (Variables|Default|SetParticleActivated true)
    (else
      (bind _returnvalue_2 (Effects|SpawnEmitteratLocation (Variables|Default|GetExplosionParticle) (Transformation|GetWorldLocation (Variables|Default|GetExplostionPointBack))))
      (Variables|Default|SetExplosionParticleRef _returnvalue_2)
      (Variables|Default|SetParticleActivated true))))

(fn StopExplosion
  (bind _explosionparticleref (Variables|Default|GetExplosionParticleRef))
  (Utilities|IsValid _explosionparticleref
    (:Is%20Valid
      (Components|Activation|Deactivate _explosionparticleref))))

(fn UpdateCarLocation
  (params (Alpha :type Float%20%28single-precision%29))
  (bind _car (Variables|Default|GetCar))
  (bind _relativelocation (Variables|/Script/Engine.SceneComponent|GetRelativeLocation _car))
  (Transformation|SetRelativeLocation _car (Math|Vector|MakeVector (Math|Float|Lerp -5e+02 5e+02 Alpha) (.y _relativelocation) (.z _relativelocation)) true false))

(fn RestartCarPosition
  (Transformation|SetRelativeLocation (Variables|Default|GetCar) (Variables|Default|GetInitialCarLocation) false false)
  (CallFunction|StopExplosion)
  (Variables|Default|SetisOnRightLane true)
  (Variables|Default|SetCanSwerve true))

(fn StartAudio
  (Audio|PlaySoundatLocation "/Game/Assets/Audio/EngineCue.EngineCue" (Transformation|GetWorldLocation (Variables|Default|GetCar))))