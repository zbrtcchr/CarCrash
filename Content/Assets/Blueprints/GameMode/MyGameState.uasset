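; Game state that drives which menu or gameplay UI is shown in an endless game.
; ChangeGameState sets NewGameState, whose RepNotify removes the old HUD UI and updates CurrentGameState, whose own RepNotify shows the new UI.
; Hardcoded parent menus support back navigation, with a special Home Menu case that cancels an active loading screen.
; Backgrounding the app clears the connecting flag and pauses a running game.
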(event Custom|OnApplicationEnterBackground
  (Variables|/Game/Assets/Blueprints/GameMode/EndlessGameMode.EndlessGameMode_C|SetIsTryingToConnect (.AsEndless%20Game%20Mode (Utilities|Casting|CastToEndlessGameMode (Game|GetGameMode))) false)
  (switch Utilities|FlowControl|Switch|SwitchonEGameState (Variables|Default|GetCurrentGameState)
    (:NewEnumerator0
      (Default|OnPauseGame (.AsEndless%20PC (Utilities|Casting|CastToEndlessPC (Game|GetPlayerController 0))))
      (Variables|Default|SetNewGameState "NewEnumerator3"))))

(event EventBeginPlay
  (EventDispatchers|BindEventtoApplicationWillEnterBackgroundDelegate (Variables|Default|GetApplicationLifecycle) (delegate Custom|OnApplicationEnterBackground)))

(fn ConstructionScript)

(fn OnRepCurrentGameState
  (Utilities|FlowControl|Sequence
    (:then_0
      (switch Utilities|FlowControl|Switch|SwitchonEGameState (Variables|Default|GetCurrentGameState)
        (:NewEnumerator5
          (Variables|Default|SetPreviousGameState "NewEnumerator1" :!label _label))
        (:NewEnumerator6
          (Variables|Default|SetPreviousGameState "NewEnumerator5"))
        (:NewEnumerator10
          (goto _label))
        (:NewEnumerator11
          (goto _label))))
    (:then_1
      (Default|SetUI (Variables|Default|GetHUDRef) (Variables|Default|GetCurrentGameState)))))

(fn OnRepNewGameState
  (Default|RemoveUI (Variables|Default|GetHUDRef) (Variables|Default|GetCurrentGameState))
  (Variables|Default|SetPreviousGameState (Variables|Default|GetCurrentGameState))
  (Variables|Default|SetCurrentGameState (Variables|Default|GetNewGameState)))

(fn ChangeGameState
  (params (NewGameState :type EGameState%20Enum))
  (Variables|Default|SetNewGameState NewGameState))

(fn ReturnPreviousState
  (bind _returnvalue (Game|GetGameMode))
  (bind _returnvalue_2 (Game|GetGameMode))
  (bind _asendless_game_mode (Utilities|Casting|CastToEndlessGameMode _returnvalue))
  (bind _asendless_game_mode_2 (Utilities|Casting|CastToEndlessGameMode _returnvalue_2))
  (bind _loadingscreen (Variables|/Game/Assets/Blueprints/GameMode/EndlessGameMode.EndlessGameMode_C|GetLoadingScreen _asendless_game_mode))
  (switch Utilities|FlowControl|Switch|SwitchonEGameState (Variables|Default|GetCurrentGameState)
    (:NewEnumerator1
      (Utilities|IsValid _loadingscreen
        (:Is%20Valid
          (if (UserInterface|Viewport|IsinViewport _loadingscreen)
            (Default|EndLoadingScreen _asendless_game_mode_2)
            (Variables|/Game/Assets/Blueprints/GameMode/EndlessGameMode.EndlessGameMode_C|SetProceed? _asendless_game_mode_2 false)
            (Viewport|RemoveAllWidgets)
            (bind _returnvalue_3 (UserInterface|CreateWidget "/Game/Assets/Blueprints/UI/WB_S_AdBanner.WB_S_AdBanner_C"))
            (UserInterface|Viewport|AddtoViewport _returnvalue_3 0)
            (CallFunction|ChangeGameState (Variables|/Game/Assets/Blueprints/GameMode/EndlessGameMode.EndlessGameMode_C|GetGameStateRef (.AsEndless%20Game%20Mode (Utilities|Casting|CastToEndlessGameMode (Game|GetGameMode)))) "NewEnumerator1")))))
    (:NewEnumerator5
      (Variables|Default|SetNewGameState (Variables|Default|GetPreviousGameState) :!label _label))
    (:NewEnumerator6
      (goto _label))
    (:NewEnumerator10
      (goto _label))
    (:NewEnumerator11
      (goto _label))))