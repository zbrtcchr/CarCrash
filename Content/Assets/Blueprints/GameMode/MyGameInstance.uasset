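; MyGameInstance is the game instance of an endless-style game, using RepNotify functions to react to changes in mute, in-app purchase and gem state.
; Mute changes swap the base sound mix, pause or play audio through EndlessPC and persist the flag.
; Purchases save online through EndlessGameMode when IsGSRegistered, otherwise through EndlessPC.
; Gem purchases add the mapped amount to CurrentGems, whose notify saves the balance.
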(fn OnRepIsMute
  (bind _returnvalue (Game|GetPlayerController 0))
  (bind _asendless_pc (Utilities|Casting|CastToEndlessPC _returnvalue))
  (bind _savegameinstance (Default|GetSaveGame _asendless_pc))
  (if (Variables|Settings|GetIsMute)
    (Class|GameplayStatics|SetBaseSoundMix "/Game/Assets/Audio/SM_Mute.SM_Mute")
    (Default|PauseAudio (.AsEndless%20PC (Utilities|Casting|CastToEndlessPC (Game|GetPlayerController 0))))
    (else
      (Class|GameplayStatics|SetBaseSoundMix "/Game/Assets/Audio/SM_Loud.SM_Loud")
      (Default|PlayAudio (.AsEndless%20PC (Utilities|Casting|CastToEndlessPC (Game|GetPlayerController 0))))))
  (Variables|/Game/Assets/Blueprints/GameMode/MyGameSave.MyGameSave_C|SetIsMute _savegameinstance (Variables|Settings|GetIsMute))
  (Default|SaveGame _asendless_pc _savegameinstance))

(fn OnRepinAppPurchase
  (bind _returnvalue (Game|GetPlayerController 0))
  (bind _asendless_pc (Utilities|Casting|CastToEndlessPC _returnvalue))
  (if (Variables|/Game/Assets/Blueprints/GameMode/MyGameSave.MyGameSave_C|GetIsGSRegistered (Default|GetSaveGame _asendless_pc))
    (Default|SaveTransactionOnline (.AsEndless%20Game%20Mode (Utilities|Casting|CastToEndlessGameMode (Game|GetGameMode))) (Variables|IAP|GetInAppPurchase))
    (else
      (Default|SaveTransaction _asendless_pc (Variables|IAP|GetInAppPurchase))))
  (switch Utilities|FlowControl|Switch|SwitchonEStoreState (Variables|IAP|GetIAPState)
    (:NewEnumerator0
      (Variables|Game|SetCurrentGems (+ (Variables|Game|GetCurrentGems) (.Value (Utilities|Map|Find (Variables|IAP|GetIAPMap) (Variables|IAP|GetIAPIdentifierStr))))))))

(fn OnRepCurrentGems
  (Default|SaveGems (.AsEndless%20PC (Utilities|Casting|CastToEndlessPC (Game|GetPlayerController 0))) (Variables|Game|GetCurrentGems)))