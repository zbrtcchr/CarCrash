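; Player controller for an endless car game with arcade modes, linking the player car, score, HUD, game state and saving.
; At BeginPlay it caches the car and SaveManager actors and passes the HUD to ScoreManager and game state.
; It gates lane switching, starts, stops and resets the car, and configures mode goals and speed.
; Victory saves arcade progress and adds a gem; most save calls simply forward to SaveManager.
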(event Custom|OnGameOver
  ;[1 1 1] On game over
  (Game|StopGame)
  (Default|ChangeGameState (Variables|Default|GetBrickGameStateRef) "NewEnumerator9"))

(event Custom|OnVictory
  ;[1 1 1] On Victory
  (Game|StopGame)
  (Default|ChangeGameState (Variables|Default|GetBrickGameStateRef) "NewEnumerator8")
  (Save/Load|SaveArcadeLevel (Variables|/Game/Assets/Blueprints/GameMode/MyGameInstance.MyGameInstance_C|GetArcadeMode (Variables|Default|GetMyGameInstRef)))
  (Variables|/Game/Assets/Blueprints/GameMode/MyGameInstance.MyGameInstance_C|SetCurrentGems (Variables|Default|GetMyGameInstRef) (+ (Variables|/Game/Assets/Blueprints/GameMode/MyGameInstance.MyGameInstance_C|GetCurrentGems (Variables|Default|GetMyGameInstRef)) 1))
  (Development|PrintString (Utilities|String|Append "Current Gems are: " (Utilities|String|ToString(Integer) (Variables|/Game/Assets/Blueprints/GameMode/MyGameInstance.MyGameInstance_C|GetCurrentGems (Variables|Default|GetMyGameInstRef)))) false))

(event Custom|OnPauseGame
  ;[1 1 1] On pause game. Called when pause button is pressed
  (Game|StopGame)
  (Variables|/Game/Assets/Blueprints/GameMode/MyGameInstance.MyGameInstance_C|SetCurrentScore (Variables|Default|GetMyGameInstRef) (Default|GetScore (Variables|Default|GetScoreManager))))

(event EventBeginPlay
  (bind _returnvalue (Game|GetGameState))
  (bind _asmy_game_state (Utilities|Casting|CastToMyGameState _returnvalue))
  ;[1 1 1] Gets reference to Player Car
  (bind _outactors (Actor|GetAllActorsOfClass "/Game/Assets/Blueprints/CarPawn/CarWithCamera.CarWithCamera_C"))
  (bind _output_get (Variables|Default|SetCarRef (Utilities|Array|Get(acopy) _outactors)))
  (Variables|Default|SetInitialCarTransform (Transformation|GetActorTransform _output_get))
  ;[1 1 1] Get referernce to EndlessHUD and pass value to ScoreManager and BrickGameState
  (bind _output_get_2 (Variables|/Game/Assets/Blueprints/ActorComponent/ScoreManager.ScoreManager_C|SetHUDRef (Variables|Default|GetScoreManager) (.AsEndless%20HUD (Utilities|Casting|CastToEndlessHUD (HUD|GetHUD)))))
  (Variables|/Game/Assets/Blueprints/GameMode/MyGameState.MyGameState_C|SetHUDRef _asmy_game_state _output_get_2)
  ;[1 1 1] Get a local reference of GameState and Game Instance
  (Variables|Default|SetBrickGameStateRef _asmy_game_state)
  (Variables|Default|SetMyGameInstRef (.AsMy%20Game%20Instance (Utilities|Casting|CastToMyGameInstance (Game|GetGameInstance))))
  (bind _outactors_2 (Actor|GetAllActorsOfClass "/Game/Assets/Blueprints/ActorComponent/SaveManager.SaveManager_C"))
  (Variables|Save|SetSaveManagerRef (Utilities|Array|Get(acopy) _outactors_2)))

(event Input|KeyboardEvents|AndroidBack
  (params (Key :type Key%20Structure :default "AnyKey"))
  ;[1 1 1] on pressing back button
  (:Pressed
    (Default|BackButtonPressed (.AsEndless%20Game%20Mode (Utilities|Casting|CastToEndlessGameMode (Game|GetGameMode))))))

(fn ConstructionScript)

(fn CheckifAddScore
  (params (ScoreChange :type Integer) (ShouldScore :type Boolean))
  (if ShouldScore
    (Default|AddScoreOnly (Variables|Default|GetScoreManager) ScoreChange)))

(fn SwitchCarPosition
  (if (Variables|Default|GetCanControl)
    (Default|ChangeRoad (Variables|Default|GetCarRef))))

(fn RestartPosition
  (Transformation|SetActorTransform (Variables|Default|GetCarRef) (Variables|Default|GetInitialCarTransform))
  (Default|OnRestart (Variables|Default|GetCarRef))
  (Default|SetScore (Variables|Default|GetScoreManager)))

(fn StartGame
  (Default|StartCar (Variables|Default|GetCarRef))
  (Variables|Default|SetCanControl true)
  (Variables|/Game/Assets/Blueprints/ActorComponent/TimerManager.TimerManager_C|SetIsPaused (Variables|/Game/Assets/Blueprints/CarPawn/CarWithCamera.CarWithCamera_C|GetTimerManager (Variables|Default|GetCarRef)) false)
  (Variables|/Game/Assets/Blueprints/GameMode/MyGameInstance.MyGameInstance_C|SetIsHighScore (Variables|Default|GetMyGameInstRef) false))

(fn StopGame
  (Default|StopCar (Variables|Default|GetCarRef))
  (Variables|Default|SetCanControl false)
  (Variables|/Game/Assets/Blueprints/ActorComponent/TimerManager.TimerManager_C|SetIsPaused (Variables|/Game/Assets/Blueprints/CarPawn/CarWithCamera.CarWithCamera_C|GetTimerManager (Variables|Default|GetCarRef)) true))

(fn GetHighScore
  (return (Default|GetHighScore (Variables|Save|GetSaveManagerRef))))

(fn SaveHighScore
  (Default|SaveHighScore (Variables|Save|GetSaveManagerRef) (Default|GetScore (Variables|Default|GetScoreManager)))
  (return))

(fn SetFinalScore
  (params (GameOverWidget :type WB%20Game%20Over%20Widget%20Object%20Reference))
  (Default|ShowFinalScore GameOverWidget (Default|GetScore (Variables|Default|GetScoreManager))))

(fn SetGameMode
  (params (MaxGoal :type Integer) (NewSpeedMultiplier :type Float%20%28single-precision%29) (NewInitialSpeed :type Float%20%28single-precision%29))
  (Default|SetMaxScore (Variables|Default|GetScoreManager) MaxGoal)
  (Default|UpdateAcceleration (Variables|/Game/Assets/Blueprints/CarPawn/CarWithCamera.CarWithCamera_C|GetSpeedManager (Variables|Default|GetCarRef)) NewSpeedMultiplier)
  (Default|UpdateSpeed (Variables|/Game/Assets/Blueprints/CarPawn/CarWithCamera.CarWithCamera_C|GetSpeedManager (Variables|Default|GetCarRef)) NewInitialSpeed))

(fn StartArcade
  (params (ArcadeState :type EArcadeMode%20Enum))
  (bind _carref (Variables|Default|GetCarRef))
  (switch Utilities|FlowControl|Switch|SwitchonEArcadeMode ArcadeState
    (:NewEnumerator2
      (Default|OnActivateTimer (Variables|/Game/Assets/Blueprints/CarPawn/CarWithCamera.CarWithCamera_C|GetTimerManager _carref) _carref))
    (:NewEnumerator3
      (Variables|/Game/Assets/Blueprints/ActorComponent/SpeedManager.SpeedManager_C|SetShouldCountSpeedScore (Variables|/Game/Assets/Blueprints/CarPawn/CarWithCamera.CarWithCamera_C|GetSpeedManager (Variables|Default|GetCarRef)) true))))

(fn SaveArcadeLevel
  (params (ArcadeMode :type EArcadeMode%20Enum))
  (Default|SaveArcadeLevel (Variables|Save|GetSaveManagerRef) ArcadeMode))

(fn GetSaveGame
  (return (Default|GetSaveGame (Variables|Save|GetSaveManagerRef))))

(fn GetArcadeLevel
  (params (ArcadeMode :type EArcadeMode%20Enum))
  (return (Default|GetArcadeLevel (Variables|Save|GetSaveManagerRef) ArcadeMode)))

(fn ContinueGame
  (bind _scoremanager (Variables|Default|GetScoreManager))
  (Transformation|SetActorTransform (Variables|Default|GetCarRef) (Variables|Default|GetInitialCarTransform))
  (Default|RestartCarPosition (Variables|Default|GetCarRef))
  (Default|SetScore _scoremanager (Default|GetScore _scoremanager)))

(fn SaveGems
  (params (CurrentGems :type Integer))
  (Default|SaveGems (Variables|Save|GetSaveManagerRef) CurrentGems))

(fn SaveGametoDevice
  (params (HIghScore :type Integer) (Gems :type Integer) (ClassicLevel :type Integer) (CrashLevel :type Integer) (SpeedLevel :type Integer) (TimerLevel :type Integer))
  (Default|SaveGamefromGS (Variables|Save|GetSaveManagerRef) HIghScore Gems ClassicLevel CrashLevel SpeedLevel TimerLevel))

(fn ShowCountdown
  (params (IsContinue :type Boolean))
  (Default|ShowCountdown (.AsEndless%20HUD (Utilities|Casting|CastToEndlessHUD (HUD|GetHUD))) IsContinue))

(fn SaveGame
  (params (SaveGameObject :type My%20Game%20Save%20Object%20Reference%20%28by%20ref%29))
  (Default|SaveGame (Variables|Save|GetSaveManagerRef) SaveGameObject))

(fn PauseAudio
  (Class|AudioComponent|SetPaused (Variables|/Game/Assets/Blueprints/CarPawn/CarWithCamera.CarWithCamera_C|GetCarEngine (Variables|Default|GetCarRef)) true))

(fn PlayAudio
  (Class|AudioComponent|SetPaused (Variables|/Game/Assets/Blueprints/CarPawn/CarWithCamera.CarWithCamera_C|GetCarEngine (Variables|Default|GetCarRef)) false))

(fn SaveTransaction
  (params (Transaction :type In%20App%20Purchase%20Info%20Struct%20Structure))
  (Default|SaveTransaction (Variables|Save|GetSaveManagerRef) Transaction))

(fn SavetoGS
  (Default|SavetoGS (Variables|Save|GetSaveManagerRef)))