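; HUD for the endless game that shows and removes its screens by game state, from title, menus and store to gameplay, pause and end screens.
; SetUI lazily creates and caches each widget, feeding some score, arcade level or game mode data, while RemoveUI detaches them.
; AddToBackOfViewport clears and re-adds widgets so new screens sit beneath existing ones, above only the countdown.
; The countdown pauses and continues with the game.
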(fn ConstructionScript)

(fn SetUI
  (params (GameState :type EGameState%20Enum))
  (bind _returnvalue (Game|GetGameInstance))
  (bind _asmy_game_instance (Utilities|Casting|CastToMyGameInstance _returnvalue))
  (switch Utilities|FlowControl|Switch|SwitchonEGameState GameState
    (:NewEnumerator0
      ;[1 1 1] Start Game
      (Utilities|FlowControl|Sequence
        (:then_0
          (Utilities|IsValid (Variables|Default|GetCountDownWidget)
            (:Is%20Valid
              (Default|ContinueCountdown (Variables|Default|GetCountDownWidget)))))
        (:then_1
          (Utilities|IsValid (Variables|Default|GetTouchInterfaceRef)
            (:Is%20Valid
              _)
            (:Is%20Not%20Valid
              (bind _returnvalue_2 (UserInterface|CreateWidget "/Game/Assets/Blueprints/UI/Screen/WB_S_GameInterface.WB_S_GameInterface_C"))
              (Variables|Default|SetTouchInterfaceRef _returnvalue_2)))
          (CallFunction|AddtoBackOfViewport (Variables|Default|GetTouchInterfaceRef)))))
    (:NewEnumerator1
      ;[1 1 1] TitleScreen
      (Utilities|IsValid (Variables|Default|GetTitleScreenRef2)
        (:Is%20Valid
          _)
        (:Is%20Not%20Valid
          (bind _returnvalue_3 (UserInterface|CreateWidget "/Game/Assets/Blueprints/UI/Screen/WB_S_Title.WB_S_Title_C"))
          (Variables|Default|SetTitleScreenRef2 _returnvalue_3)))
      (Variables|/Game/Assets/Blueprints/UI/Screen/WB_S_Title.WB_S_Title_C|SetGMRef (Variables|Default|GetTitleScreenRef2) (.AsEndless%20Game%20Mode (Utilities|Casting|CastToEndlessGameMode (Game|GetGameMode))))
      (CallFunction|AddtoBackOfViewport (Variables|Default|GetTitleScreenRef2))
      (Utilities|IsValid (Variables|Default|GetCountDownWidget)
        (:Is%20Valid
          (Widget|RemovefromParent (Variables|Default|GetCountDownWidget)))))
    (:NewEnumerator3
      ;[1 1 1] Pause Game
      (Utilities|FlowControl|Sequence
        (:then_0
          (Utilities|IsValid (Variables|Default|GetCountDownWidget)
            (:Is%20Valid
              (Default|PauseCountdown (Variables|Default|GetCountDownWidget)))))
        (:then_1
          (Utilities|IsValid (Variables|Default|GetPauseMenuRef)
            (:Is%20Valid
              _)
            (:Is%20Not%20Valid
              (bind _returnvalue_4 (UserInterface|CreateWidget "/Game/Assets/Blueprints/UI/Screen/WB_S_PauseMenu.WB_S_PauseMenu_C"))
              (Variables|Default|SetPauseMenuRef _returnvalue_4)))
          (CallFunction|UpdateScore (Variables|/Game/Assets/Blueprints/GameMode/MyGameInstance.MyGameInstance_C|GetCurrentScore (.AsMy%20Game%20Instance (Utilities|Casting|CastToMyGameInstance (Game|GetGameInstance)))))
          (CallFunction|AddtoBackOfViewport (Variables|Default|GetPauseMenuRef)))))
    (:NewEnumerator4
      ;[1 1 1] Game Over
      (Utilities|IsValid (Variables|Default|GetGameEndIntRef2)
        (:Is%20Valid
          _)
        (:Is%20Not%20Valid
          (bind _returnvalue_5 (UserInterface|CreateWidget "/Game/Assets/Blueprints/UI/Screen/WB_S_GameEnd.WB_S_GameEnd_C"))
          (Variables|Default|SetGameEndIntRef2 _returnvalue_5)))
      (Default|SetFinalScore (.AsEndless%20PC (Utilities|Casting|CastToEndlessPC (Variables|Default|GetPlayerOwner))) (Variables|/Game/Assets/Blueprints/UI/Screen/WB_S_GameEnd.WB_S_GameEnd_C|GetGameOverWidget (Variables|Default|GetGameEndIntRef2)))
      (CallFunction|AddtoBackOfViewport (Variables|Default|GetGameEndIntRef2)))
    (:NewEnumerator5
      ;[1 1 1] Choose Game Mode
      (Utilities|IsValid (Variables|Default|GetChooseGameModeRef)
        (:Is%20Valid
          _)
        (:Is%20Not%20Valid
          (bind _returnvalue_6 (UserInterface|CreateWidget "/Game/Assets/Blueprints/UI/Screen/WB_S_ChooseGameMode.WB_S_ChooseGameMode_C"))
          (Variables|Default|SetChooseGameModeRef _returnvalue_6)))
      (CallFunction|AddtoBackOfViewport (Variables|Default|GetChooseGameModeRef)))
    (:NewEnumerator6
      ;[1 1 1] Choose Arcade
      (Utilities|IsValid (Variables|Default|GetChooseArcadeMode)
        (:Is%20Valid
          _)
        (:Is%20Not%20Valid
          (bind _returnvalue_7 (UserInterface|CreateWidget "/Game/Assets/Blueprints/UI/Screen/WB_S_ChooseArcade.WB_S_ChooseArcade_C"))
          (Variables|Default|SetChooseArcadeMode _returnvalue_7)))
      (CallFunction|SetLevels)
      (Variables|/Game/Assets/Blueprints/UI/Screen/WB_S_ChooseArcade.WB_S_ChooseArcade_C|SetGMRef (Variables|Default|GetChooseArcadeMode) (.AsEndless%20Game%20Mode (Utilities|Casting|CastToEndlessGameMode (Game|GetGameMode))))
      (CallFunction|AddtoBackOfViewport (Variables|Default|GetChooseArcadeMode)))
    (:NewEnumerator7
      ;[1 1 1] Tutorial Screen
      (Utilities|IsValid (Variables|Default|GetTutorialScreenRef)
        (:Is%20Valid
          _)
        (:Is%20Not%20Valid
          (bind _returnvalue_8 (UserInterface|CreateWidget "/Game/Assets/Blueprints/UI/Screen/WB_S_Tutorial.WB_S_Tutorial_C"))
          (Variables|Default|SetTutorialScreenRef _returnvalue_8)))
      (CallFunction|AddtoBackOfViewport (Variables|Default|GetTutorialScreenRef)))
    (:NewEnumerator8
      ;[1 1 1] Victory Screen
      (Utilities|IsValid (Variables|Default|GetVictoryScreenRef2)
        (:Is%20Valid
          _)
        (:Is%20Not%20Valid
          (bind _returnvalue_9 (UserInterface|CreateWidget "/Game/Assets/Blueprints/UI/Screen/WB_S_Victory.WB_S_Victory_C"))
          (Variables|Default|SetVictoryScreenRef2 _returnvalue_9)))
      (Default|SetArcadeInfo (Variables|/Game/Assets/Blueprints/UI/Screen/WB_S_Victory.WB_S_Victory_C|GetArcadeSlot_108 (Variables|Default|GetVictoryScreenRef2)) (Variables|/Game/Assets/Blueprints/GameMode/MyGameInstance.MyGameInstance_C|GetArcadeMode _asmy_game_instance) (Variables|/Game/Assets/Blueprints/GameMode/MyGameInstance.MyGameInstance_C|GetArcadeLevel _asmy_game_instance))
      (Variables|/Game/Assets/Blueprints/UI/Screen/WB_S_Victory.WB_S_Victory_C|SetArcadeMode (Variables|Default|GetVictoryScreenRef2) (Variables|/Game/Assets/Blueprints/GameMode/MyGameInstance.MyGameInstance_C|GetArcadeMode _asmy_game_instance))
      (CallFunction|AddtoBackOfViewport (Variables|Default|GetVictoryScreenRef2)))
    (:NewEnumerator9
      ;[1 1 1] Continue
      (Utilities|IsValid (Variables|Default|GetContinueScreen)
        (:Is%20Valid
          _)
        (:Is%20Not%20Valid
          (bind _returnvalue_10 (UserInterface|CreateWidget "/Game/Assets/Blueprints/UI/Screen/WB_S_Continue.WB_S_Continue_C"))
          (Variables|Default|SetContinueScreen _returnvalue_10)))
      (Default|SetFinalScore (.AsEndless%20PC (Utilities|Casting|CastToEndlessPC (Variables|Default|GetPlayerOwner))) (Variables|/Game/Assets/Blueprints/UI/Screen/WB_S_Continue.WB_S_Continue_C|GetGameOverWidget (Variables|Default|GetContinueScreen)))
      (CallFunction|AddtoBackOfViewport (Variables|Default|GetContinueScreen)))
    (:NewEnumerator10
      ;[1 1 1] Leaderboard
      (Utilities|IsValid (Variables|Default|GetLeaderboardScreenRef)
        (:Is%20Valid
          _)
        (:Is%20Not%20Valid
          (bind _returnvalue_11 (UserInterface|CreateWidget "/Game/Assets/Blueprints/UI/Screen/WB_S_Leaderboard.WB_S_Leaderboard_C"))
          (Variables|Default|SetLeaderboardScreenRef _returnvalue_11)))
      (CallFunction|AddtoBackOfViewport (Variables|Default|GetLeaderboardScreenRef)))
    (:NewEnumerator11
      ;[1 1 1] Settings
      (Utilities|IsValid (Variables|Default|GetSettingsScreenRef)
        (:Is%20Valid
          _)
        (:Is%20Not%20Valid
          (bind _returnvalue_12 (UserInterface|CreateWidget "/Game/Assets/Blueprints/UI/Screen/WB_S_Settings.WB_S_Settings_C"))
          (Variables|Default|SetSettingsScreenRef _returnvalue_12)))
      (CallFunction|AddtoBackOfViewport (Variables|Default|GetSettingsScreenRef)))
    (:NewEnumerator12
      ;[1 1 1] Store
      (Utilities|IsValid (Variables|Default|GetStoreRef)
        (:Is%20Valid
          _)
        (:Is%20Not%20Valid
          (bind _returnvalue_13 (UserInterface|CreateWidget "/Game/Assets/Blueprints/UI/Screen/WB_S_Store.WB_S_Store_C" 0 false))
          (Variables|Default|SetStoreRef _returnvalue_13)))
      (CallFunction|AddtoBackOfViewport (Variables|Default|GetStoreRef)))))

(fn UpdateScore
  (params (NewScore :type Integer))
  (bind _touchinterfaceref (Variables|Default|GetTouchInterfaceRef))
  (Utilities|IsValid _touchinterfaceref
    (:Is%20Valid
      (Default|SetScore (Variables|/Game/Assets/Blueprints/UI/Screen/WB_S_GameInterface.WB_S_GameInterface_C|GetScoreInterface _touchinterfaceref) NewScore))))

(fn SetLevels
  (bind _asendless_pc (Utilities|Casting|CastToEndlessPC (Game|GetPlayerController 0)))
  (bind _arcadelevel (Default|GetArcadeLevel _asendless_pc "NewEnumerator0"))
  (LocalVariables|SetClassicLevelLoc _arcadelevel)
  (bind _arcadelevel_2 (Default|GetArcadeLevel _asendless_pc "NewEnumerator1"))
  (LocalVariables|SetCrashLevelLoc _arcadelevel_2)
  (bind _arcadelevel_3 (Default|GetArcadeLevel _asendless_pc "NewEnumerator2"))
  (LocalVariables|SetTimerLevelLoc _arcadelevel_3)
  (bind _arcadelevel_4 (Default|GetArcadeLevel _asendless_pc "NewEnumerator3"))
  (LocalVariables|SetSpeedLevelLoc _arcadelevel_4)
  (Default|SetTextBlockLevels (Variables|Default|GetChooseArcadeMode) (LocalVariables|GetClassicLevelLoc) (LocalVariables|GetCrashLevelLoc) (LocalVariables|GetTimerLevelLoc) (LocalVariables|GetSpeedLevelLoc)))

(fn ShowCountdown
  (params (IsContinue :type Boolean))
  (Utilities|IsValid (Variables|Default|GetCountDownWidget)
    (:Is%20Valid
      _)
    (:Is%20Not%20Valid
      (bind _returnvalue (UserInterface|CreateWidget "/Game/Assets/Blueprints/UI/Widgets/WB_CountDownWidget.WB_CountDownWidget_C"))
      (Variables|Default|SetCountDownWidget _returnvalue)))
  (Default|OnConstruct (Variables|Default|GetCountDownWidget) IsContinue)
  (UserInterface|Viewport|AddtoViewport (Variables|Default|GetCountDownWidget) 0)
  (Default|StartCountdown (Variables|Default|GetCountDownWidget)))

(fn RemoveifValid
  (params (InputObject :type User%20Widget%20Object%20Reference))
  (Utilities|FlowControl|Sequence
    (:then_0
      (Utilities|IsValid InputObject
        (:Is%20Valid
          (Widget|RemovefromParent InputObject))))
    (:then_1
      (return))))

(fn RemoveUI
  (params (GameState :type EGameState%20Enum))
  (switch Utilities|FlowControl|Switch|SwitchonEGameState GameState
    (:NewEnumerator0
      (CallFunction|RemoveifValid (Variables|Default|GetTouchInterfaceRef)))
    (:NewEnumerator1
      (CallFunction|RemoveifValid (Variables|Default|GetTitleScreenRef2)))
    (:NewEnumerator3
      (CallFunction|RemoveifValid (Variables|Default|GetPauseMenuRef)))
    (:NewEnumerator4
      (CallFunction|RemoveifValid (Variables|Default|GetGameEndIntRef2)))
    (:NewEnumerator5
      (CallFunction|RemoveifValid (Variables|Default|GetChooseGameModeRef)))
    (:NewEnumerator6
      (CallFunction|RemoveifValid (Variables|Default|GetChooseArcadeMode)))
    (:NewEnumerator7
      (CallFunction|RemoveifValid (Variables|Default|GetTutorialScreenRef)))
    (:NewEnumerator8
      (CallFunction|RemoveifValid (Variables|Default|GetVictoryScreenRef2)))
    (:NewEnumerator9
      (CallFunction|RemoveifValid (Variables|Default|GetContinueScreen)))
    (:NewEnumerator10
      (CallFunction|RemoveifValid (Variables|Default|GetLeaderboardScreenRef)))
    (:NewEnumerator11
      (CallFunction|RemoveifValid (Variables|Default|GetSettingsScreenRef)))
    (:NewEnumerator12
      (CallFunction|RemoveifValid (Variables|Default|GetStoreRef)))))

(fn IsUIActive
  (params (WidgetToCheck :type User%20Widget%20Object%20Reference))
  (return (UserInterface|Viewport|IsinViewport WidgetToCheck)))

(fn AddtoBackOfViewport
  (params (WidgetToAdd :type User%20Widget%20Object%20Reference))
  (bind _countdownwidget (Variables|Default|GetCountDownWidget))
  (bind _foundwidgets (Widget|GetAllWidgetsOfClass "/Script/UMG.UserWidget" true))
  (bind _output_get (LocalVariables|SetAllWidgetsLocal _foundwidgets))
  (Viewport|RemoveAllWidgets)
  (if (Utilities|Array|ContainsItem _output_get _countdownwidget)
    (UserInterface|Viewport|AddtoViewport _countdownwidget 0)
    (Utilities|Array|RemoveItem (LocalVariables|GetAllWidgetsLocal) _countdownwidget))
  (UserInterface|Viewport|AddtoViewport WidgetToAdd 0)
  (Utilities|Array|RemoveItem (LocalVariables|GetAllWidgetsLocal) WidgetToAdd)
  (if (> (Utilities|Array|Length (LocalVariables|GetAllWidgetsLocal)) 0)
    (for _array_element (LocalVariables|GetAllWidgetsLocal)
      (UserInterface|Viewport|AddtoViewport _array_element 0))))