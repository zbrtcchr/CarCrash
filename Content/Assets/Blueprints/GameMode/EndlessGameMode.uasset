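; Game mode for an endless tile-based car runner with endless play and four arcade variants (Classic, Crash, Timer, Speed).
; Spawns floor tiles chained by attach transforms, tuned per mode, and drives start, restart, continue and scoring through EndlessPC.
; Also handles online features: GameSparks connection with Facebook login, cloud save and load, and sequentially fetched global and friends leaderboards.
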(event OnGameSparksAvailableDelegate(GameSparks)
  (params (available :type Boolean))
  ;[1 1 1] Delegates
  ;;[1 1 1] Gamesparks connect response
  (if available
    ;;;[1 0.9726 0] TODO: Link nodes
    (if (and (Variables|Leaderboard|GetProceed?) (Variables|Default|GetIsTryingToConnect))
      (Variables|Default|SetIsTryingToConnect false)
      (Online|Authenticate))
    (elif (Variables|Default|GetIsTryingToConnect)
      (Variables|Default|SetIsTryingToConnect false)
      (UI|EndLoadingScreen)
      (UI|ShowWarningScreen "Connection to leaderboard server was not made" "" false false))))

(event Custom|OnRestartGame
  ;[1 1 1] Restarts level
  (Game|RestartAll)
  (Default|ShowCountdown (Variables|GameModes|GetPCRef) false)
  (Default|StartGame (Variables|GameModes|GetPCRef)))

(event Custom|GetLeaderboardData
  ;[1 1 1] Get leaderboard data from gamesparks
  (Utilities|GetNewLeaderboardData "NewEnumerator0"
    (:Completed
      (Utilities|GetNewLeaderboardData "NewEnumerator1"
        (:Completed
          (Utilities|GetNewLeaderboardData "NewEnumerator2"
            (:Completed
              (bind _logeventresponse (|SendLogEventRequest "GET_ME" 0 false)
                (:OnResponse
                  (Default|UpdateMeData (Variables|Components|GetLeaderboardUMGManager) (Class|GameSparksScriptData|GetNumber (Class|GameSparksScriptData|GetGSData (Class|GameSparksScriptData|GetGSData (.ScriptData (Utilities|Struct|BreakGSLogEventResponse _logeventresponse)) "MeData") "meGlobalData") "HIGHSCORE") (Class|GameSparksScriptData|GetNumber (Class|GameSparksScriptData|GetGSData (Class|GameSparksScriptData|GetGSData (.ScriptData (Utilities|Struct|BreakGSLogEventResponse _logeventresponse)) "MeData") "meGlobalData") "RANK") (Class|GameSparksScriptData|GetString (Class|GameSparksScriptData|GetGSData (Class|GameSparksScriptData|GetGSData (.ScriptData (Utilities|Struct|BreakGSLogEventResponse _logeventresponse)) "MeData") "meGlobalData") "USERNAME") true)
                  (Default|UpdateMeData (Variables|Components|GetLeaderboardUMGManager) (Class|GameSparksScriptData|GetNumber (Class|GameSparksScriptData|GetGSData (Class|GameSparksScriptData|GetGSData (.ScriptData (Utilities|Struct|BreakGSLogEventResponse _logeventresponse)) "MeData") "meFriendsData") "HIGHSCORE") (Class|GameSparksScriptData|GetNumber (Class|GameSparksScriptData|GetGSData (Class|GameSparksScriptData|GetGSData (.ScriptData (Utilities|Struct|BreakGSLogEventResponse _logeventresponse)) "MeData") "meFriendsData") "RANK") (Class|GameSparksScriptData|GetString (Class|GameSparksScriptData|GetGSData (Class|GameSparksScriptData|GetGSData (.ScriptData (Utilities|Struct|BreakGSLogEventResponse _logeventresponse)) "MeData") "meFriendsData") "USERNAME") false)
                  (Default|ChangeGameState (Variables|GameModes|GetGameStateRef) "NewEnumerator10")
                  ;[1 1 1] Event to remove loading screen from screen
                  (UI|EndLoadingScreen))))))))))

(event Custom|ContinueFacebookRegistration
  ;[1 1 1] Gets leaderboard data
  (CallFunction|LoadGamefromCloud)
  (|SendLogEventRequest "SAVE_HIGHSCORE" (Class|GameSparksLogEventData|SetNumber (Class|GameSparksLogEventData|CreateGameSparksLogEventAttributes) "HIGHSCORE" (UI|GetHighScore)) false
    (:then
      (if (Variables|Leaderboard|GetGoToLeaderboard)
        (CallFunction|GetLeaderboardData)
        (else
          (UI|EndLoadingScreen))))))

(event Custom|LoadGameFromCloud
  ;[1 1 1] Load game data from cloud to device
  (bind _logeventresponse (|SendLogEventRequest "LOAD_RUNTIME" 0 false)
    (:OnResponse
      (Default|SaveGametoDevice (Variables|GameModes|GetPCRef) (Class|GameSparksScriptData|GetNumber (Class|GameSparksScriptData|GetGSData (.ScriptData (Utilities|Struct|BreakGSLogEventResponse _logeventresponse)) "GAMEDATA") "HIGHSCORE") (Class|GameSparksScriptData|GetNumber (Class|GameSparksScriptData|GetGSData (.ScriptData (Utilities|Struct|BreakGSLogEventResponse _logeventresponse)) "GAMEDATA") "CLASSIC") (Class|GameSparksScriptData|GetNumber (Class|GameSparksScriptData|GetGSData (.ScriptData (Utilities|Struct|BreakGSLogEventResponse _logeventresponse)) "GAMEDATA") "CRASH") (Class|GameSparksScriptData|GetNumber (Class|GameSparksScriptData|GetGSData (.ScriptData (Utilities|Struct|BreakGSLogEventResponse _logeventresponse)) "GAMEDATA") "SPEED") (Class|GameSparksScriptData|GetNumber (Class|GameSparksScriptData|GetGSData (.ScriptData (Utilities|Struct|BreakGSLogEventResponse _logeventresponse)) "GAMEDATA") "TIMER") (Class|GameSparksScriptData|GetNumber (Class|GameSparksScriptData|GetGSData (.ScriptData (Utilities|Struct|BreakGSLogEventResponse _logeventresponse)) "GAMEDATA") "CREDITS"))
      (Online|SetLeaderboardRegistered (Class|GameSparksScriptData|GetString (Class|GameSparksScriptData|GetGSData (.ScriptData (Utilities|Struct|BreakGSLogEventResponse _logeventresponse)) "GAMEDATA") "USERID")))))

(event Custom|OnStartEndless
  ;[1 1 1] Start endless game from choose game mode screen
  (Game|SetEndlessGameMode)
  (Default|ShowCountdown (Variables|GameModes|GetPCRef) false)
  (Default|StartGame (Variables|GameModes|GetPCRef)))

(event Custom|FacebookAuthenticate
  (params (AccessToken :type String))
  ;[1 1 1] Authenticates facebook to Gameparks
  (bind (_authenticationresponse _haserrors) (|SendFacebookConnectRequest AccessToken "" false false 0 false false 0 false)
    (:OnResponse
      (if _haserrors
        ;;[1 1 1] Authentication failure
        (UI|EndLoadingScreen)
        (UI|ShowWarningScreen "There was an error registering to the leaderboard" "" false false)
        (Class|FacebookforUnrealBPLibrary|FacebookLogout)
        (else
          (Variables|/Game/Assets/Blueprints/GameMode/MyGameInstance.MyGameInstance_C|SetIsFbLoggedIn (.AsMy%20Game%20Instance (Utilities|Casting|CastToMyGameInstance (Game|GetGameInstance))) true)
          (UI|ShowWarningScreen "YOU HAVE CONNECTED SUCCESSFULLY." "" false false "FACEBOOK LOGIN")
          (if (.NewPlayer (Utilities|Struct|BreakGSAuthenticationResponse _authenticationresponse))
            ;[1 1 1] Gets leaderboard data
            (Online|SetLeaderboardRegistered (.UserId (Utilities|Struct|BreakGSAuthenticationResponse _authenticationresponse)))
            (else
              (Utilities|CheckUserId (.UserId (Utilities|Struct|BreakGSAuthenticationResponse _authenticationresponse)) (.DisplayName (Utilities|Struct|BreakGSAuthenticationResponse _authenticationresponse))
                (:Continue
                  (CallFunction|LoadGamefromCloud)))))
          (|SendLogEventRequest "SAVE_HIGHSCORE" (Class|GameSparksLogEventData|SetNumber (Class|GameSparksLogEventData|CreateGameSparksLogEventAttributes) "HIGHSCORE" (UI|GetHighScore)) false
            (:then
              (if (Variables|Leaderboard|GetGoToLeaderboard)
                (CallFunction|GetLeaderboardData)
                (else
                  (UI|EndLoadingScreen))))))))))

(event Custom|OnStartArcade
  (params (ArcadeMode :type EArcadeMode%20Enum))
  ;[1 1 1] Start Arcade mode
  (bind _output_get (Variables|Game|SetArcadeState ArcadeMode))
  (bind _arcadelevel (Default|GetArcadeLevel (Variables|GameModes|GetPCRef) _output_get))
  (Variables|Game|SetArcadeLevel _arcadelevel)
  (Game|SetArcadeGameMode)
  (Game|RestartAll)
  (Default|ShowCountdown (Variables|GameModes|GetPCRef) false)
  (Default|StartGame (Variables|GameModes|GetPCRef)))

(event Custom|OnChooseGameMode
  ;[1 1 1] Go to Choose Game Mode Screen
  (Default|ChangeGameState (Variables|GameModes|GetGameStateRef) "NewEnumerator5"))

(event Custom|OnBeginGame
  ;[1 1 1] On Begin Game
  (Game|SpawnTiles)
  (Default|ChangeGameState (Variables|GameModes|GetGameStateRef) "NewEnumerator1")
  (Default|StopGame (Variables|GameModes|GetPCRef)))

(event Custom|SaveGameToCloud
  (params (SaveGameInstance :type My%20Game%20Save%20Object%20Reference))
  ;[1 1 1] Save game data from device to Cloud
  (|SendLogEventRequest "SAVE_RUNTIME" (Class|GameSparksLogEventData|SetNumber (Class|GameSparksLogEventData|SetNumber (Class|GameSparksLogEventData|SetNumber (Class|GameSparksLogEventData|SetNumber (Class|GameSparksLogEventData|SetNumber (Class|GameSparksLogEventData|SetNumber (Class|GameSparksLogEventData|CreateGameSparksLogEventAttributes) "CLASSIC" (Variables|/Game/Assets/Blueprints/GameMode/MyGameSave.MyGameSave_C|GetClassicLevel SaveGameInstance)) "CRASH" (Variables|/Game/Assets/Blueprints/GameMode/MyGameSave.MyGameSave_C|GetCrashLevel SaveGameInstance)) "SPEED" (Variables|/Game/Assets/Blueprints/GameMode/MyGameSave.MyGameSave_C|GetSpeedLevel SaveGameInstance)) "TIMER" (Variables|/Game/Assets/Blueprints/GameMode/MyGameSave.MyGameSave_C|GetTimerLevel SaveGameInstance)) "CREDITS" (Variables|/Game/Assets/Blueprints/GameMode/MyGameSave.MyGameSave_C|GetCredits SaveGameInstance)) "HIGHSCORE" (Variables|/Game/Assets/Blueprints/GameMode/MyGameSave.MyGameSave_C|GetHighScore SaveGameInstance)) false))

(event Custom|OnContinueGame
  ;[1 1 1] On Continuing game from game over
  (Variables|Game|SetNextAttachPoint (Math|Transform|MakeTransform "0, 0,0.000000"))
  (Default|ContinueGame (Variables|GameModes|GetPCRef))
  (Game|RemoveAllTiles)
  (Game|SpawnTiles)
  (Default|ShowCountdown (Variables|GameModes|GetPCRef) true))

(event Custom|OnGoHome
  ;[1 1 1] Pressing home screen button - All tiles will lead to endless game unless arcade game is selected
  (Game|SetEndlessGameMode)
  (Game|RestartAll)
  (Default|StopGame (Variables|GameModes|GetPCRef))
  (Class|AdCollectionBPLibrary|ShowBanner "AdMob" true))

(event Custom|OnPauseGame
  ;[1 1 1] Pause game
  (Default|OnPauseGame (Variables|GameModes|GetPCRef)))

(event Custom|FbLogin
  ;[1 1 1] Facebook login
  (bind _accesstoken (|FacebookLogin)
    (:OnSuccess
      (CallFunction|FacebookAuthenticate _accesstoken))))

(event Custom|OnContinueFinishedCountdown
  ;[1 1 1] On Continuing game from game over
  ;;[1 1 1] When Countdown after pressing continue finished
  (Default|StartGame (Variables|GameModes|GetPCRef)))

(event Custom|OnScreenTouch
  ;[1 1 1] On touch on touch interface
  (Default|SwitchCarPosition (Variables|GameModes|GetPCRef)))

(event Custom|BackButtonPressed
  ;[1 1 1] Called when back button is pressed
  (Default|ReturnPreviousState (Variables|GameModes|GetGameStateRef)))

(event EventBeginPlay
  (Variables|GameModes|SetGameStateRef (.AsMy%20Game%20State (Utilities|Casting|CastToMyGameState (Game|GetGameState))))
  (Variables|GameModes|SetPCRef (.AsEndless%20PC (Utilities|Casting|CastToEndlessPC (Game|GetPlayerController 0))))
  (CallFunction|OnBeginGame)
  (if (Variables|/Game/Assets/Blueprints/GameMode/MyGameSave.MyGameSave_C|GetIsFacebookRegistered (Default|GetSaveGame (Variables|GameModes|GetPCRef)))
    (GameSparks|ConnectOnline false)))

(event EventEndPlay
  (params (EndPlayReason :type EEndPlayReason%20Enum :default "Destroyed"))
  ;[1 1 1] Event End Play
  (GameSparks|GSDisconnect))

(fn ConstructionScript)

(fn AddFloorTile
  (params (NextTileClass :type Floor%20Tile%20Class%20Reference) (CurrentTileClass :type Floor%20Tile%20Class%20Reference) (ShouldSpawn :type Boolean))
  (LocalVariables|SetNewTileLoc NextTileClass)
  (LocalVariables|SetCurrentTileLoc CurrentTileClass)
  (LocalVariables|SetShouldSpawnLoc ShouldSpawn)
  (if (Variables|/Game/Assets/Blueprints/GameMode/MyGameInstance.MyGameInstance_C|GetIsEndless (.AsMy%20Game%20Instance (Utilities|Casting|CastToMyGameInstance (Game|GetGameInstance))))
    (Game|SpawnFloorTile (LocalVariables|GetNewTileLoc) (LocalVariables|GetCurrentTileLoc) (LocalVariables|GetShouldSpawnLoc) true true 0.01 1.0)
    (else
      (switch Utilities|FlowControl|Switch|SwitchonEArcadeMode (Variables|Game|GetArcadeState)
        (:NewEnumerator0
          (Game|SpawnFloorTile (LocalVariables|GetNewTileLoc) (LocalVariables|GetCurrentTileLoc) (LocalVariables|GetShouldSpawnLoc) true false 0.01 1.0))
        (:NewEnumerator1
          (Game|SpawnFloorTile (LocalVariables|GetNewTileLoc) (LocalVariables|GetCurrentTileLoc) (LocalVariables|GetShouldSpawnLoc) false true (Utilities|Struct|BreakArcadeConditionsStruct (Variables|Game|GetArcadeConditions)) 1.0))
        (:NewEnumerator2
          (Game|SpawnFloorTile (LocalVariables|GetNewTileLoc) (LocalVariables|GetCurrentTileLoc) (LocalVariables|GetShouldSpawnLoc) false false 0.01 1.0))
        (:NewEnumerator3
          (Game|SpawnFloorTile (LocalVariables|GetNewTileLoc) (LocalVariables|GetCurrentTileLoc) (LocalVariables|GetShouldSpawnLoc) false false 0.01 (Utilities|Struct|BreakArcadeConditionsStruct (Variables|Game|GetArcadeConditions))))))))

(fn OnPassingScoreTile
  (params (FloorScore :type Integer) (ShouldScore :type Boolean))
  (Default|CheckifAddScore (Variables|GameModes|GetPCRef) FloorScore ShouldScore))

(fn SpawnTiles
  (for _index (range 0 (- (LocalVariables|GetNumberOfSpawns) 1))
    (if (== (Math|Integer|%(Integer) _index 2) 0)
      (Game|AddFloorTile "/Game/Assets/Blueprints/FloorTile/FloorTile.FloorTile_C" "/Game/Assets/Blueprints/FloorTile/FloorTile.FloorTile_C" true)
      (else
        (Game|AddFloorTile "/Game/Assets/Blueprints/FloorTile/FloorTile.FloorTile_C" "/Game/Assets/Blueprints/FloorTile/CarTile.CarTile_C" true)))))

(fn RemoveAllTiles
  (bind _outactors (Actor|GetAllActorsOfClass "/Game/Assets/Blueprints/FloorTile/FloorTile.FloorTile_C"))
  (for _array_element _outactors
    (Actor|DestroyActor _array_element)))

(fn RepositionFloorTile
  (params (Tile :type Floor%20Tile%20Object%20Reference))
  (Transformation|SetActorTransform Tile (Variables|Game|GetNextAttachPoint))
  (Variables|Game|SetNextAttachPoint (Default|GetAttachTransform Tile)))

(fn RestartAll
  (bind _returnvalue (Game|GetGameInstance))
  (bind _asmy_game_instance (Utilities|Casting|CastToMyGameInstance _returnvalue))
  (Variables|Game|SetNextAttachPoint (Math|Transform|MakeTransform "0, 0, 0"))
  (Default|RestartPosition (Variables|GameModes|GetPCRef))
  (Game|RemoveAllTiles)
  (Game|SpawnTiles)
  (Variables|/Game/Assets/Blueprints/GameMode/MyGameInstance.MyGameInstance_C|SetIsVideoWatched _asmy_game_instance false)
  (Variables|/Game/Assets/Blueprints/GameMode/MyGameInstance.MyGameInstance_C|SetNumberOfContinues _asmy_game_instance 0))

(fn GetHighScore
  (bind _highscore (Default|GetHighScore (Variables|GameModes|GetPCRef)))
  (return _highscore))

(fn OnPassingScorePoint
  (params (PointScore :type Integer))
  (Default|AddScoreOnly (Variables|/Game/Assets/Blueprints/GameMode/EndlessPC.EndlessPC_C|GetScoreManager (Variables|GameModes|GetPCRef)) PointScore))

(fn SpawnFloorTile
  (params (NextTileClass :type Floor%20Tile%20Class%20Reference) (CurrentTile :type Floor%20Tile%20Class%20Reference) (ShouldSpawn :type Boolean) (ShouldCountFloorScore :type Boolean) (ShouldCountPointScore :type Boolean) (PointChance :type Float%20%28single-precision%29) (FloorScale :type Float%20%28single-precision%29))
  (bind _returnvalue (Game|SpawnActorfromClass NextTileClass (Variables|Game|GetNextAttachPoint) "Undefined" 0 CurrentTile ShouldSpawn PointChance FloorScale ShouldCountFloorScore ShouldCountPointScore))
  (Variables|Game|SetNextAttachPoint (Default|GetAttachTransform _returnvalue)))

(fn SetEndlessGameMode
  (bind _arcadeconditions (Variables|Game|GetArcadeConditions))
  (bind (_accelerationnormal _initialspeedendless) (Utilities|Struct|BreakArcadeConditionsStruct _arcadeconditions))
  (Variables|/Game/Assets/Blueprints/GameMode/MyGameInstance.MyGameInstance_C|SetIsEndless (.AsMy%20Game%20Instance (Utilities|Casting|CastToMyGameInstance (Game|GetGameInstance))) true)
  (Variables|/Game/Assets/Blueprints/ActorComponent/TimerManager.TimerManager_C|SetShouldCountTimeScore (Variables|/Game/Assets/Blueprints/CarPawn/CarWithCamera.CarWithCamera_C|GetTimerManager (Variables|/Game/Assets/Blueprints/GameMode/EndlessPC.EndlessPC_C|GetCarRef (Variables|GameModes|GetPCRef))) false)
  (Variables|/Game/Assets/Blueprints/ActorComponent/SpeedManager.SpeedManager_C|SetShouldCountSpeedScore (Variables|/Game/Assets/Blueprints/CarPawn/CarWithCamera.CarWithCamera_C|GetSpeedManager (Variables|/Game/Assets/Blueprints/GameMode/EndlessPC.EndlessPC_C|GetCarRef (Variables|GameModes|GetPCRef))) false)
  (Default|SetGameMode (Variables|GameModes|GetPCRef) 0 _accelerationnormal _initialspeedendless))

(fn SetArcadeGameMode
  (bind _arcadeconditions (Variables|Game|GetArcadeConditions))
  (bind _arcadeconditions_2 (Variables|Game|GetArcadeConditions))
  (bind _pcref (Variables|GameModes|GetPCRef))
  (bind _arcadeconditions_3 (Variables|Game|GetArcadeConditions))
  (bind _arcadeconditions_4 (Variables|Game|GetArcadeConditions))
  (bind (_accelerationfast _initialspeedendless _speedmaxgoal) (Utilities|Struct|BreakArcadeConditionsStruct _arcadeconditions))
  (bind (_accelerationfast_2 _initialspeedendless_2 _timermaxgoal) (Utilities|Struct|BreakArcadeConditionsStruct _arcadeconditions_2))
  (bind (_accelerationnormal _initialspeedendless_3 _classicmaxgoal) (Utilities|Struct|BreakArcadeConditionsStruct _arcadeconditions_4))
  (bind (_accelerationfast_3 _initialspeedendless_4 _crashmaxgoal) (Utilities|Struct|BreakArcadeConditionsStruct _arcadeconditions_3))
  (switch Utilities|FlowControl|Switch|SwitchonEArcadeMode (Variables|Game|GetArcadeState)
    (:NewEnumerator0
      (Default|SetGameMode (Variables|GameModes|GetPCRef) (+ _classicmaxgoal (* (Variables|Game|GetArcadeLevel) 5)) _accelerationnormal _initialspeedendless_3))
    (:NewEnumerator1
      (Default|SetGameMode (Variables|GameModes|GetPCRef) (+ _crashmaxgoal (* (Variables|Game|GetArcadeLevel) 5)) _accelerationfast_3 _initialspeedendless_4))
    (:NewEnumerator2
      (Default|SetGameMode _pcref (+ _timermaxgoal (* (Variables|Game|GetArcadeLevel) 3)) _accelerationfast_2 _initialspeedendless_2)
      (Default|TimerSetProperties (Variables|/Game/Assets/Blueprints/CarPawn/CarWithCamera.CarWithCamera_C|GetTimerManager (Variables|/Game/Assets/Blueprints/GameMode/EndlessPC.EndlessPC_C|GetCarRef _pcref))))
    (:NewEnumerator3
      (Default|SetGameMode (Variables|GameModes|GetPCRef) (+ _speedmaxgoal (* (Variables|Game|GetArcadeLevel) 5)) _accelerationfast _initialspeedendless)))
  (bind _asmy_game_instance (Utilities|Casting|CastToMyGameInstance (Game|GetGameInstance)))
  (Variables|/Game/Assets/Blueprints/GameMode/MyGameInstance.MyGameInstance_C|SetArcadeLevel _asmy_game_instance (Variables|Game|GetArcadeLevel))
  (Variables|/Game/Assets/Blueprints/GameMode/MyGameInstance.MyGameInstance_C|SetArcadeMode _asmy_game_instance (Variables|Game|GetArcadeState))
  (Variables|/Game/Assets/Blueprints/GameMode/MyGameInstance.MyGameInstance_C|SetIsEndless _asmy_game_instance false))

(fn SpawnDefaultPawnfor
  (params (NewPlayer :type Controller%20Object%20Reference) (StartSpot :type Actor%20Object%20Reference))
  (return 0))

(fn GSDisconnect
  (Class|GameSparksComponent|Disconnect (Variables|Components|GetGameSparks)))

(fn Authenticate
  (if (Class|FacebookforUnrealBPLibrary|IsFacebookLoggedin)
    (CallFunction|FacebookAuthenticate (Class|FacebookforUnrealBPLibrary|GetFacebookAccessToken))
    (elif (Variables|Leaderboard|GetGoToLeaderboard)
      (if (Variables|Leaderboard|GetProceed?)
        (UI|ShowLoginWarningScreen))
      (else
        (CallFunction|FbLogin)))))

(fn ShowWarningScreen
  (params (Message :type Text) (PlayerName :type String) (IsTwoOptions :type Boolean) (IsFinal :type Boolean) (Header :type Text))
  (LocalVariables|SetMessageLoc Message)
  (LocalVariables|SetIsTwoOptionsLoc IsTwoOptions)
  (LocalVariables|SetPlayerNameLoc PlayerName)
  (LocalVariables|SetIsFinalLoc IsFinal)
  (LocalVariables|SetHeaderLoc Header)
  (bind _returnvalue (UserInterface|CreateWidget "/Game/Assets/Blueprints/UI/WB_S_Warning.WB_S_Warning_C" 0 (LocalVariables|GetMessageLoc) (LocalVariables|GetIsTwoOptionsLoc) (LocalVariables|GetPlayerNameLoc) (LocalVariables|GetIsFinalLoc) (LocalVariables|GetHeaderLoc)))
  (UserInterface|Viewport|AddtoViewport _returnvalue 0))

(fn ShowLoginWarningScreen
  (bind _returnvalue (UserInterface|CreateWidget "/Game/Assets/Blueprints/UI/WB_S_Login.WB_S_Login_C"))
  (UserInterface|Viewport|AddtoViewport _returnvalue 0))

(fn ConnectOnline
  (params (GoToLeaderboard :type Boolean))
  (Variables|Leaderboard|SetGoToLeaderboard GoToLeaderboard)
  (Variables|Leaderboard|SetProceed? true)
  (Variables|Default|SetIsTryingToConnect true)
  (bind _returnvalue (Class|GameSparksComponent|IsAvailable (Variables|Components|GetGameSparks)))
  (if _returnvalue
    (Online|Authenticate)
    (else
      (Class|GameSparksComponent|Connect (Variables|Components|GetGameSparks) "d316060snfwU" "YgKhy14FgZ7XbP2jlDPXKwbMPCezs5Gz" true false))))

(fn SetLeaderboardRegistered
  (params (UserId :type String))
  (LocalVariables|SetSaveGameInstanceLoc (Default|GetSaveGame (Variables|GameModes|GetPCRef)))
  (Variables|/Game/Assets/Blueprints/GameMode/MyGameSave.MyGameSave_C|SetRegisteredGSUserId (LocalVariables|GetSaveGameInstanceLoc) UserId)
  (Variables|/Game/Assets/Blueprints/GameMode/MyGameSave.MyGameSave_C|SetIsFacebookRegistered (LocalVariables|GetSaveGameInstanceLoc) true)
  (Default|SaveGame (Variables|GameModes|GetPCRef) (LocalVariables|GetSaveGameInstanceLoc)))

(fn OpenLoadingScreen
  (Utilities|IsValid (Variables|UI|GetLoadingScreen)
    (:Is%20Valid
      _)
    (:Is%20Not%20Valid
      (bind _returnvalue (UserInterface|CreateWidget "/Game/Assets/Blueprints/UI/WB_LoadingScreen.WB_LoadingScreen_C"))
      (Variables|UI|SetLoadingScreen _returnvalue)))
  (UserInterface|Viewport|AddtoViewport (Variables|UI|GetLoadingScreen) 0))

(fn EndLoadingScreen
  (Widget|RemovefromParent (Variables|UI|GetLoadingScreen)))

(fn GetImageLink
  (params (ShareAction :type EActionType%20Enum) (IsHighScore :type Boolean))
  (switch Utilities|FlowControl|Switch|SwitchonEActionType ShareAction
    (:ACTION_PLAYS
      (return (Variables|Facebook|GetFb_ImageLink_Plays)))
    (:ACTION_CELEBRATE
      (if IsHighScore
        (return (Variables|Facebook|GetFb_ImageLink_HighScore))
        (else
          (return (Variables|Facebook|GetFb_ImageLink_ArcadeFinish)))))))