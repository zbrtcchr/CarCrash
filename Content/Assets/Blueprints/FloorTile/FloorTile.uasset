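; FloorTile is a road segment for an endless car game, scaled along X with its attach point and end trigger placed from the mesh length.
; When the player's car overlaps the end trigger, a "Car"-tagged component reports the tile's score to EndlessGameMode once, sometimes with a horn.
; A "Reposition"-tagged component asks the game mode to add the next tile or recycle this one, depending on ShouldSpawn.
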(event OnComponentBeginOverlap(TileEndTrigger)
  (params (OverlappedComponent :type Primitive%20Component%20Object%20Reference) (OtherActor :type Actor%20Object%20Reference) (OtherComp :type Primitive%20Component%20Object%20Reference) (OtherBodyIndex :type Integer) (bFromSweep :type Boolean) (SweepResult :type Hit%20Result%20Structure%20%28by%20ref%29))
  (Utilities|Casting|CastToCarWithCamera OtherActor)
  (Variables|Default|SetGameModeRef (.AsEndless%20Game%20Mode (Utilities|Casting|CastToEndlessGameMode (Game|GetGameMode))))
  (Utilities|FlowControl|Sequence
    (:then_0
      (CallFunction|CheckifShouldScore OtherComp))
    (:then_1
      (CallFunction|SpawnorReposition OtherComp))))

(fn ConstructionScript
  (bind _tileendtrigger (Variables|Default|GetTileEndTrigger))
  (bind _floortile (Variables|Default|GetFloorTile))
  (bind _returnvalue (Transformation|GetWorldScale _floortile))
  (bind _returnvalue_2 (* (.x _returnvalue) -1.4e+03))
  (Components|StaticMesh|SetStaticMesh (Variables|Default|GetFloorTile) (Variables|Default|GetFloorTileMesh))
  (Transformation|SetRelativeScale3D (Variables|Default|GetFloorTile) (Math|Vector|MakeVector (Variables|Default|GetFloorScale) 1.0 1.0))
  (Transformation|SetRelativeLocation (Variables|Default|GetAttachPoint) (Math|Vector|MakeVector _returnvalue_2 0.0 0.0) false false)
  (Transformation|SetRelativeLocation _tileendtrigger (Math|Vector|MakeVector (+ _returnvalue_2 (.x (Variables|/Script/Engine.BoxComponent|GetBoxExtent _tileendtrigger))) 0.0 225.0) false false))

(fn GetAttachTransform
  (return (Transformation|GetWorldTransform (Variables|Default|GetAttachPoint))))

(fn RepositionSelf
  (params (GameMode :type Endless%20Game%20Mode%20Object%20Reference) (Floor%20Tile :type Floor%20Tile%20Object%20Reference))
  (Default|RepositionFloorTile GameMode Floor%20Tile))

(fn CheckifShouldScore
  (params (OtherComponent :type Actor%20Component%20Object%20Reference))
  (if (Math|Boolean|ANDBoolean (not (Variables|Default|GetIsPassedByCar)) (Components|ComponentHasTag OtherComponent "Car") (!= (Variables|Default|GetFloorScore) 0))
    (Default|OnPassingScoreTile (Variables|Default|GetGameModeRef) (Variables|Default|GetFloorScore) (Variables|Default|GetShouldCountFloorScore))
    (Variables|Default|SetIsPassedByCar true)
    (if (Math|Random|RandomBoolwithWeight 0.35)
      (Audio|PlaySoundatLocation "/Game/Assets/Audio/Car/Horn/CarHorn.CarHorn" (Variables|Default|GetCarHornLocation)))))

(fn SpawnorReposition
  (params (OtherComponent :type Actor%20Component%20Object%20Reference))
  (bind _gamemoderef (Variables|Default|GetGameModeRef))
  (if (Components|ComponentHasTag OtherComponent "Reposition")
    (if (Variables|Default|GetShouldSpawn)
      (Default|AddFloorTile _gamemoderef (Variables|Default|GetNextTileClass) (Variables|Default|GetCurrentTileClass) false)
      (else
        (CallFunction|RepositionSelf _gamemoderef self)))))