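; Floor tile carrying an obstacle car, re-randomized whenever the tile is recycled through the GameMode.
; Each car gets a random side and type: blue point, yellow moving or red enemy.
; Yellow cars switch sides via a Timeline lerp when the player's car enters MoveTrigger.
; Collisions spawn a front or back explosion with crash audio; blue cars also vanish and can score once per recycle.
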(event OnComponentBeginOverlap(MoveTrigger)
  (params (OverlappedComponent :type Primitive%20Component%20Object%20Reference) (OtherActor :type Actor%20Object%20Reference) (OtherComp :type Primitive%20Component%20Object%20Reference) (OtherBodyIndex :type Integer) (bFromSweep :type Boolean) (SweepResult :type Hit%20Result%20Structure%20%28by%20ref%29))
  (bind _obstacle (Variables|Default|GetObstacle))
  (bind _relativelocation (Variables|/Script/Engine.SceneComponent|GetRelativeLocation _obstacle))
  (bind (_x _y _z) (Math|Vector|BreakVector _relativelocation))
  (Utilities|Casting|CastToCarWithCamera OtherActor)
  (if (Math|Boolean|ANDBoolean (Variables|Default|GetObstacleMoves) (not (Variables|Default|GetFinishedMoving)) (Components|ComponentHasTag OtherComp "Car"))
    (if (Variables|Default|GetIsOnRight)
      (bind _fasteralpha (Timeline|Timeline_0 PlayFromStart)
        (:Update
          (Transformation|SetRelativeLocation (Variables|Default|GetObstacle) (Math|Vector|MakeVector _x (Math|Float|Lerp -5e+02 5e+02 _fasteralpha) _z) true false)
          (Variables|Default|SetFinishedMoving true)))
      (else
        (Timeline|Timeline_0 ReverseFromEnd)))))

(event Custom|OnCollisionWithCar
  (params (OnFront :type Boolean))
  (CallFunction|StartExplosion OnFront)
  (if (Variables|Default|GetIsObstaclePoint)
    (Rendering|SetVisibility (Variables|Default|GetObstacle) false true)
    (if (Variables|Default|GetShouldCountPointScore)
      (Default|OnPassingScorePoint (Variables|Default|GetGameModeRef) (Variables|Default|GetPointScore))
      (Variables|Default|SetShouldCountPointScore false))))

(event EventBeginPlay
  (Variables|Default|SetCarHornLocation (Transformation|GetWorldLocation (Variables|CarTile_C|GetCarHorn self))))

(event EventRepositionSelf
  (params (GameMode :type Endless%20Game%20Mode%20Object%20Reference) (Floor%20Tile :type Floor%20Tile%20Object%20Reference))
  (Default|RepositionFloorTile GameMode Floor%20Tile)
  (CallFunction|RepositionObstacle (Variables|Default|GetObstacle))
  (CallFunction|RandomizeCar)
  (Variables|Default|SetIsPassedByCar false))

(fn ConstructionScript
  (|CallParentFunction)
  (Components|StaticMesh|SetStaticMesh (Variables|Default|GetObstacle) (Variables|Default|GetObstacleMesh))
  (CallFunction|RepositionObstacle (Variables|Default|GetObstacle))
  (CallFunction|RandomizeCar))

(fn RepositionObstacle
  (params (Obstacle%20Ref :type Scene%20Component%20Object%20Reference))
  (if (Math|Random|RandomBool)
    (Transformation|SetRelativeLocation Obstacle%20Ref (Math|Vector|MakeVector -6.4e+02 5e+02 1.6e+02) false false)
    (Variables|Default|SetIsOnRight false)
    (else
      (Transformation|SetRelativeLocation Obstacle%20Ref (Math|Vector|MakeVector -6.4e+02 -5e+02 1.6e+02) false false)
      (Variables|Default|SetIsOnRight true)))
  (Rendering|SetVisibility (Variables|Default|GetObstacle) true true))

(fn StartExplosion
  (params (OnFront :type Boolean))
  (bind _carhorn (Variables|Default|GetCarHorn))
  (if OnFront
    (Effects|SpawnEmitteratLocation (Variables|Default|GetExplosionParticle) (Transformation|GetWorldLocation (Variables|Default|GetExplosionPointFront)) "0,0.000000, 0")
    (else
      (Effects|SpawnEmitteratLocation (Variables|Default|GetExplosionParticle) (Transformation|GetWorldLocation (Variables|Default|GetExplosionPointBack)) "0,0.000000, 0")))
  (Audio|Components|Audio|SetSound _carhorn "/Game/Assets/Audio/Explosion/Crash-Cue.Crash-Cue")
  (Audio|Components|Audio|Play _carhorn 0.0))

(fn RandomizeCar
  (bind _obstacle (Variables|Default|GetObstacle))
  (bind _obstacle_2 (Variables|Default|GetObstacle))
  (bind _obstacle_3 (Variables|Default|GetObstacle))
  (if (< (Math|Random|RandomFloatinRange 0.0 1.0) (Variables|Default|GetPointChance))
    ;[1 1 1] Blue
    (Variables|Default|SetIsObstaclePoint true)
    (Components|StaticMesh|SetStaticMesh _obstacle_2 (Variables|Default|GetObstacleMesh))
    (Rendering|Material|SetMaterial _obstacle_2 0 "/Game/Assets/Materials/MaterialInstances/MI_CarPoint.MI_CarPoint")
    (else
      (Variables|Default|SetIsObstaclePoint false)
      (bind _output_get (Variables|Default|SetObstacleMoves (< (Math|Random|RandomFloatinRange 0.0 1.0) (LocalVariables|GetYellowCarChance))))
      (Variables|Default|SetFinishedMoving false)
      (if _output_get
        ;[1 1 1] Yellow
        (Components|StaticMesh|SetStaticMesh _obstacle_3 (Variables|Default|GetObstacleMesh))
        (Rendering|Material|SetMaterial _obstacle_3 0 "/Game/Assets/Materials/MaterialInstances/MI_CarMoving.MI_CarMoving")
        (else
          ;[1 1 1] Red
          (Components|StaticMesh|SetStaticMesh _obstacle (Variables|Default|GetObstacleMesh))
          (Rendering|Material|SetMaterial _obstacle 0 "/Game/Assets/Materials/MaterialInstances/MI_CarEnemy.MI_CarEnemy")))))
  (Variables|Default|SetShouldCountPointScore (Variables|Default|GetShouldCountPointScoreInitial)))