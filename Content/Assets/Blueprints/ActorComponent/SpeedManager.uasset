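; Actor component that drives its owner forward in an endless car mode, starting at the game mode's arcade initial speed.
; While movement is allowed, each Tick offsets the owner along local Y by Speed, unscaled by delta time, then accelerates toward a maximum.
; Speed gains below the cap feed an optional SpeedScore, whose RepNotify updates the ScoreManager.
; Setting speed to zero stops the CarWithCamera, and Restart resets speed and score counting.
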(event EventTick
  (params (DeltaSeconds :type Float%20%28single-precision%29))
  (if (Variables|CarControl|GetCanMove)
    (CallFunction|MoveForward)
    (CallFunction|ComputeSpeed DeltaSeconds)))

(event EventBeginPlay
  (bind _asendless_game_mode (Utilities|Casting|CastToEndlessGameMode (Game|GetGameMode)))
  (bind _output_get (Variables|Properties|SetSpeed (Utilities|Struct|BreakArcadeConditionsStruct (Variables|/Game/Assets/Blueprints/GameMode/EndlessGameMode.EndlessGameMode_C|GetArcadeConditions _asendless_game_mode))))
  (CallFunction|UpdateSpeed _output_get))

(fn GetSpeed
  (return (Variables|Properties|GetSpeed)))

(fn MoveForward
  (Transformation|AddActorLocalOffset (Components|GetOwner) (Math|Vector|MakeVector 0.0 (Variables|Properties|GetSpeed) 0.0) false false))

(fn ComputeSpeed
  (params (SpeedDelta :type Float%20%28single-precision%29%20%28by%20ref%29))
  (bind _maxspeed (Variables|Default|GetMaxSpeed))
  (bind _speed (Variables|Properties|GetSpeed))
  (bind _acceleration (Variables|CarControl|GetAcceleration))
  (bind _returnvalue (* SpeedDelta _acceleration))
  (bind _returnvalue_2 (+ _returnvalue _speed))
  (if (> _returnvalue_2 _maxspeed)
    (CallFunction|UpdateSpeed _maxspeed)
    (else
      (CallFunction|UpdateSpeed _returnvalue_2)
      (CallFunction|ComputeSpeedScore _returnvalue))))

(fn UpdateSpeed
  (params (NewSpeed :type Float%20%28single-precision%29%20%28by%20ref%29))
  (Variables|Properties|SetSpeed NewSpeed)
  (if (== NewSpeed 0.0)
    (bind _ascar_with_camera (Utilities|Casting|CastToCarWithCamera (Components|GetOwner)))
    (Default|StopCar _ascar_with_camera)))

(fn UpdateAcceleration
  (params (NewSpeedMultiplier :type Float%20%28single-precision%29))
  (Variables|CarControl|SetAcceleration NewSpeedMultiplier))

(fn OnRepSpeedScore
  (Default|SetScore (Variables|/Game/Assets/Blueprints/GameMode/EndlessPC.EndlessPC_C|GetScoreManager (Variables|Default|GetPCRef)) (Math|Float|Truncate (Variables|SpeedforScore|GetSpeedScore))))

(fn ComputeSpeedScore
  (params (SpeedScoreChange :type Float%20%28single-precision%29))
  (if (Variables|SpeedforScore|GetShouldCountSpeedScore)
    (Variables|SpeedforScore|SetSpeedScore (+ SpeedScoreChange (Variables|SpeedforScore|GetSpeedScore)))))

(fn Restart
  (params (InitialSpeed :type Float%20%28single-precision%29))
  (Variables|Properties|SetSpeed InitialSpeed)
  (Variables|SpeedforScore|SetShouldCountSpeedScore false)
  (Variables|SpeedforScore|SetSpeedScore 0.0))