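; TimerManager is an actor component that scores the time a car spends in a randomly chosen scoring lane.
; While active and unpaused, Tick adds delta time to RightTimer or LeftTimer whenever the car is in that lane.
; RepNotify functions push the truncated timer to the ScoreManager through PCRef.
; TimerSetProperties picks the lane, shares it with MyGameInstance and resets both timers, which deactivation also clears.
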(event EventTick
  (params (DeltaSeconds :type Float%20%28single-precision%29))
  (if (and (Variables|Default|GetShouldCountTimeScore) (not (Variables|Default|GetIsPaused)))
    (CallFunction|ComputeTimerScore DeltaSeconds)))

(fn OnActivateTimer
  (params (CarRef :type Car%20with%20Camera%20Object%20Reference))
  (Variables|Default|SetShouldCountTimeScore true)
  (Variables|Default|SetCarRef CarRef))

(fn ComputeTimerScore
  (params (DeltaSeconds :type Float%20%28single-precision%29))
  (bind _carref (Variables|Default|GetCarRef))
  (bind _isonrightlane (Variables|/Game/Assets/Blueprints/CarPawn/CarWithCamera.CarWithCamera_C|GetisOnRightLane _carref))
  (if (Variables|Default|GetCountRightLaneAsScore)
    (if _isonrightlane
      (Variables|Default|SetRightTimer (+ DeltaSeconds (Variables|Default|GetRightTimer)))
      (return))
    (elif (not _isonrightlane)
      (Variables|Default|SetLeftTimer (+ DeltaSeconds (Variables|Default|GetLeftTimer)))
      (return))))

(fn OnRepLeftTimer
  (Default|SetScore (Variables|/Game/Assets/Blueprints/GameMode/EndlessPC.EndlessPC_C|GetScoreManager (Variables|Default|GetPCRef)) (Math|Float|Truncate (Variables|Default|GetLeftTimer))))

(fn OnRepRightTimer
  (Default|SetScore (Variables|/Game/Assets/Blueprints/GameMode/EndlessPC.EndlessPC_C|GetScoreManager (Variables|Default|GetPCRef)) (Math|Float|Truncate (Variables|Default|GetRightTimer))))

(fn AddDeltatoScore
  (params (Delta :type Float%20%28single-precision%29) (Score :type Float%20%28single-precision%29))
  (bind _output_get (Variables|Default|SetLeftTimer (+ Delta Score)))
  (return _output_get))

(fn OnDeactivate
  (Variables|Default|SetShouldCountTimeScore false)
  (Variables|Default|SetLeftTimer 0.0)
  (Variables|Default|SetRightTimer 0.0))

(fn TimerSetProperties
  (bind _output_get (Variables|Default|SetCountRightLaneAsScore (Math|Random|RandomBool)))
  (Variables|/Game/Assets/Blueprints/GameMode/MyGameInstance.MyGameInstance_C|SetTimerIsOnRightLane (.AsMy%20Game%20Instance (Utilities|Casting|CastToMyGameInstance (Game|GetGameInstance))) _output_get)
  (Variables|Default|SetLeftTimer 0.0)
  (Variables|Default|SetRightTimer 0.0))