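; SavingManager is an actor component that persists high score, gems and per-mode arcade levels in a MyGameSave slot.
; GetSaveGame loads or creates the save, and setters update it, keeping only higher scores and capping gems.
; Score, level and gem saves call SaveToGS, which pushes data and queued transactions through EndlessGameMode when registered and online.
; SaveGameFromGS overwrites local values with supplied ones, while SaveTransaction only queues locally.
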(event EventBeginPlay
  (Variables|Default|SetGameInstanceRef (.AsMy%20Game%20Instance (Utilities|Casting|CastToMyGameInstance (Game|GetGameInstance))))
  (Variables|Default|SetGameModeRef (.AsEndless%20Game%20Mode (Utilities|Casting|CastToEndlessGameMode (Game|GetGameMode)))))

(fn GetSaveGame
  (bind _returnvalue (SaveGame|DoesSaveGameExist (Variables|Default|GetSaveGameSlot) (Variables|Default|GetUserIndex)))
  (if _returnvalue
    (bind _returnvalue_2 (SaveGame|LoadGamefromSlot (Variables|Default|GetSaveGameSlot) (Variables|Default|GetUserIndex)))
    (bind _asmy_game_save (Utilities|Casting|CastToMyGameSave _returnvalue_2)
      (:then
        (Variables|Default|SetSaveGameInstance _asmy_game_save)
        (Development|PrintString "Save game exists" false)
        (Development|PrintString "Loaded save game" false)
        (return (Variables|Default|GetSaveGameInstance)))
      (:CastFailed
        (Development|PrintString "Cast to MyGameSave failed" false)))
    (else
      (bind _returnvalue_3 (SaveGame|CreateSaveGameObject "/Game/Assets/Blueprints/GameMode/MyGameSave.MyGameSave_C"))
      (Variables|Default|SetSaveGameInstance _returnvalue_3)
      (Development|PrintString "Save game does not exist" false)
      (Development|PrintString "Created save game" false)
      (return (Variables|Default|GetSaveGameInstance)))))

(fn GetHighScore
  (return (Variables|/Game/Assets/Blueprints/GameMode/MyGameSave.MyGameSave_C|GetHighScore (CallFunction|GetSaveGame))))

(fn GetArcadeLevel
  (params (ArcadeMode :type EArcadeMode%20Enum))
  (switch Utilities|FlowControl|Switch|SwitchonEArcadeMode ArcadeMode
    (:NewEnumerator0
      (return (Variables|/Game/Assets/Blueprints/GameMode/MyGameSave.MyGameSave_C|GetClassicLevel (CallFunction|GetSaveGame))))
    (:NewEnumerator1
      (return (Variables|/Game/Assets/Blueprints/GameMode/MyGameSave.MyGameSave_C|GetCrashLevel (CallFunction|GetSaveGame))))
    (:NewEnumerator2
      (return (Variables|/Game/Assets/Blueprints/GameMode/MyGameSave.MyGameSave_C|GetTimerLevel (CallFunction|GetSaveGame))))
    (:NewEnumerator3
      (return (Variables|/Game/Assets/Blueprints/GameMode/MyGameSave.MyGameSave_C|GetSpeedLevel (CallFunction|GetSaveGame))))))

(fn SaveHighScore
  (params (New%20Score :type Integer))
  (LocalVariables|SetNewScoreLoc New%20Score)
  (bind _output_get (Variables|Default|SetSaveGameInstance (CallFunction|GetSaveGame)))
  (bind _output_get_2 (LocalVariables|SetIsHighScoreLoc (> (LocalVariables|GetNewScoreLoc) (Variables|/Game/Assets/Blueprints/GameMode/MyGameSave.MyGameSave_C|GetHighScore _output_get))))
  (if _output_get_2
    (Variables|/Game/Assets/Blueprints/GameMode/MyGameSave.MyGameSave_C|SetHighScore (Variables|Default|GetSaveGameInstance) (LocalVariables|GetNewScoreLoc))
    (CallFunction|SaveGame (Variables|Default|GetSaveGameInstance))
    (Variables|/Game/Assets/Blueprints/GameMode/MyGameInstance.MyGameInstance_C|SetIsHighScore (.AsMy%20Game%20Instance (Utilities|Casting|CastToMyGameInstance (Game|GetGameInstance))) (LocalVariables|GetIsHighScoreLoc)))
  (CallFunction|SavetoGS)
  (return))

(fn SaveArcadeLevel
  (params (Arcade%20Mode :type EArcadeMode%20Enum))
  (bind _output_get (Variables|Default|SetSaveGameInstance (CallFunction|GetSaveGame)))
  (switch Utilities|FlowControl|Switch|SwitchonEArcadeMode Arcade%20Mode
    (:NewEnumerator0
      (Variables|/Game/Assets/Blueprints/GameMode/MyGameSave.MyGameSave_C|SetClassicLevel (Variables|Default|GetSaveGameInstance) (+ (Variables|/Game/Assets/Blueprints/GameMode/MyGameSave.MyGameSave_C|GetClassicLevel _output_get) 1)))
    (:NewEnumerator1
      (Variables|/Game/Assets/Blueprints/GameMode/MyGameSave.MyGameSave_C|SetCrashLevel (Variables|Default|GetSaveGameInstance) (+ (Variables|/Game/Assets/Blueprints/GameMode/MyGameSave.MyGameSave_C|GetCrashLevel _output_get) 1)))
    (:NewEnumerator2
      (Variables|/Game/Assets/Blueprints/GameMode/MyGameSave.MyGameSave_C|SetTimerLevel (Variables|Default|GetSaveGameInstance) (+ (Variables|/Game/Assets/Blueprints/GameMode/MyGameSave.MyGameSave_C|GetTimerLevel _output_get) 1)))
    (:NewEnumerator3
      (Variables|/Game/Assets/Blueprints/GameMode/MyGameSave.MyGameSave_C|SetSpeedLevel (Variables|Default|GetSaveGameInstance) (+ (Variables|/Game/Assets/Blueprints/GameMode/MyGameSave.MyGameSave_C|GetSpeedLevel _output_get) 1))))
  (CallFunction|SaveGame (Variables|Default|GetSaveGameInstance))
  (CallFunction|SavetoGS))

(fn SaveGems
  (params (CurrentGems :type Integer))
  (LocalVariables|SetCurrentGemsLoc CurrentGems)
  (Variables|Default|SetSaveGameInstance (CallFunction|GetSaveGame))
  (if (>= (LocalVariables|GetCurrentGemsLoc) (LocalVariables|GetMaxGemsLoc))
    (Variables|/Game/Assets/Blueprints/GameMode/MyGameSave.MyGameSave_C|SetGems (Variables|Default|GetSaveGameInstance) (LocalVariables|GetMaxGemsLoc))
    (else
      (Variables|/Game/Assets/Blueprints/GameMode/MyGameSave.MyGameSave_C|SetGems (Variables|Default|GetSaveGameInstance) (LocalVariables|GetCurrentGemsLoc))))
  (CallFunction|SaveGame (Variables|Default|GetSaveGameInstance))
  (Development|PrintString (Utilities|String|Append "New gems are now: " (Utilities|String|ToString(Integer) (Variables|/Game/Assets/Blueprints/GameMode/MyGameSave.MyGameSave_C|GetGems (Variables|Default|GetSaveGameInstance)))) false)
  (CallFunction|SavetoGS))

(fn SaveGame
  (params (SaveGameObject :type My%20Game%20Save%20Object%20Reference%20%28by%20ref%29))
  (bind _returnvalue (SaveGame|SaveGametoSlot SaveGameObject (Variables|Default|GetSaveGameSlot) (Variables|Default|GetUserIndex)))
  (if _returnvalue
    (Development|PrintString "SAVING GAME SUCCESSFUL" false)
    (else
      (Development|PrintString "SAVING GAME FAILED" false))))

(fn SaveGamefromGS
  (params (HighScore :type Integer) (Gems :type Integer) (ClassicLevel :type Integer) (CrashLevel :type Integer) (SpeedLevel :type Integer) (TimerLevel :type Integer))
  (Variables|Default|SetSaveGameInstance (CallFunction|GetSaveGame))
  (Variables|/Game/Assets/Blueprints/GameMode/MyGameSave.MyGameSave_C|SetHighScore (Variables|Default|GetSaveGameInstance) HighScore)
  (Variables|/Game/Assets/Blueprints/GameMode/MyGameSave.MyGameSave_C|SetGems (Variables|Default|GetSaveGameInstance) Gems)
  (Variables|/Game/Assets/Blueprints/GameMode/MyGameSave.MyGameSave_C|SetClassicLevel (Variables|Default|GetSaveGameInstance) ClassicLevel)
  (Variables|/Game/Assets/Blueprints/GameMode/MyGameSave.MyGameSave_C|SetCrashLevel (Variables|Default|GetSaveGameInstance) CrashLevel)
  (Variables|/Game/Assets/Blueprints/GameMode/MyGameSave.MyGameSave_C|SetSpeedLevel (Variables|Default|GetSaveGameInstance) SpeedLevel)
  (Variables|/Game/Assets/Blueprints/GameMode/MyGameSave.MyGameSave_C|SetTimerLevel (Variables|Default|GetSaveGameInstance) TimerLevel)
  (CallFunction|SaveGame (Variables|Default|GetSaveGameInstance)))

(fn SavetoGS
  (bind _savegameinstance (CallFunction|GetSaveGame))
  (bind _transactionsarray (Variables|/Game/Assets/Blueprints/GameMode/MyGameSave.MyGameSave_C|GetTransactionsArray _savegameinstance))
  (if (and (Variables|/Game/Assets/Blueprints/GameMode/MyGameSave.MyGameSave_C|GetIsGSRegistered (CallFunction|GetSaveGame)) (Class|FacebookforUnrealBPLibrary|IsInternetConnected))
    (Default|SaveGametoCloud (.AsEndless%20Game%20Mode (Utilities|Casting|CastToEndlessGameMode (Game|GetGameMode))) (CallFunction|GetSaveGame))
    (if (> (Utilities|Array|Length _transactionsarray) 0)
      (for _array_element _transactionsarray
        (Default|SaveTransactionOnline (.AsEndless%20Game%20Mode (Utilities|Casting|CastToEndlessGameMode (Game|GetGameMode))) _array_element))
      (Utilities|Array|Clear _transactionsarray))))

(fn SaveTransaction
  (params (Transactions :type In%20App%20Purchase%20Info%20Struct%20Structure))
  (bind _output_get (Variables|Default|SetSaveGameInstance (CallFunction|GetSaveGame)))
  (LocalVariables|SetTransactionArrayLoc (Variables|/Game/Assets/Blueprints/GameMode/MyGameSave.MyGameSave_C|GetTransactionsArray _output_get))
  (Utilities|Array|Add (LocalVariables|GetTransactionArrayLoc) Transactions)
  (Variables|/Game/Assets/Blueprints/GameMode/MyGameSave.MyGameSave_C|SetTransactionsArray (Variables|Default|GetSaveGameInstance) (LocalVariables|GetTransactionArrayLoc))
  (CallFunction|SaveGame (Variables|Default|GetSaveGameInstance))
  (if (and (Variables|/Game/Assets/Blueprints/GameMode/MyGameSave.MyGameSave_C|GetIsGSRegistered (Variables|Default|GetSaveGameInstance)) (Class|FacebookforUnrealBPLibrary|IsInternetConnected))
    _))