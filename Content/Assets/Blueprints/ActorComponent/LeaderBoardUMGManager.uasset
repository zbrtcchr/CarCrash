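; LeaderBoardUMGManager is an actor component that stores leaderboard data, by its name for UMG display.
; It keeps three lists of score, rank and name items (Global-Top, Global-Me and Friends), with add and clear functions that switch on the target list.
; The player's own entry is stored separately for global and friends boards, selected by a boolean in UpdateMeData.
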(fn AddtoList
  (params (Score :type Integer) (Rank :type Integer) (PlayerName :type String) (ListToAddDataTo :type ELeaderboardState%20Enum))
  (switch Utilities|FlowControl|Switch|SwitchonELeaderboardState ListToAddDataTo
    (:NewEnumerator0
      (Utilities|Array|Add (Variables|Default|GetGlobalList) (Utilities|Struct|MakeLeaderboardItem Score Rank PlayerName)))
    (:NewEnumerator1
      (Utilities|Array|Add (Variables|Default|GetGlobalMeList) (Utilities|Struct|MakeLeaderboardItem Score Rank PlayerName)))
    (:NewEnumerator2
      (Utilities|Array|Add (Variables|Default|GetFriendsList) (Utilities|Struct|MakeLeaderboardItem Score Rank PlayerName)))))

(fn ClearList
  (params (ListToClear :type ELeaderboardState%20Enum))
  (switch Utilities|FlowControl|Switch|SwitchonELeaderboardState ListToClear
    (:NewEnumerator0
      (Utilities|Array|Clear (Variables|Default|GetGlobalList)))
    (:NewEnumerator1
      (Utilities|Array|Clear (Variables|Default|GetGlobalMeList)))
    (:NewEnumerator2
      (Utilities|Array|Clear (Variables|Default|GetFriendsList)))))

(fn UpdateMeData
  (params (Score :type Integer) (Rank :type Integer) (Name :type String) (IsGlobal :type Boolean))
  (if IsGlobal
    (Variables|Default|SetMeData_Global (Utilities|Struct|MakeLeaderboardItem Score Rank Name))
    (else
      (Variables|Default|SetMeData_Friends (Utilities|Struct|MakeLeaderboardItem Score Rank Name)))))