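; ScoreManager is an actor component on the EndlessPC player controller that tracks score against an optional goal.
; Add, set and show functions write CurrentScore, whose RepNotify refreshes the HUD and checks the goal; ShowScore reassigns the same value to re-trigger it.
; Reaching MaxScore calls OnVictory on the owner, while zero means endless mode.
; SetMaxScore updates the touch interface's goal widget, creating that interface if missing.
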(fn AddScoreOnly
  (params (ScoreChange :type Integer))
  (Variables|Default|SetCurrentScore (+ ScoreChange (Variables|Default|GetCurrentScore))))

(fn OnRepCurrentScore
  (Default|UpdateScore (Variables|Default|GetHUDRef) (Variables|Default|GetCurrentScore))
  (CallFunction|CheckGoal))

(fn SetScore
  (params (%20NewScore :type Integer))
  (Variables|Default|SetCurrentScore %20NewScore))

(fn ShowScore
  (Variables|Default|SetCurrentScore (Variables|Default|GetCurrentScore)))

(fn GetScore
  (return (Variables|Default|GetCurrentScore)))

(fn CheckGoal
  (bind _maxscore (Variables|Default|GetMaxScore))
  (if (and (>= (Variables|Default|GetCurrentScore) _maxscore) (!= _maxscore 0)) ; If true victory\n\nElse continue
    (Default|OnVictory (.AsEndless%20PC (Utilities|Casting|CastToEndlessPC (Components|GetOwner))))))

(fn SetMaxScore
  (params (NewMaxScore :type Integer))
  (bind _hudref (Variables|Default|GetHUDRef))
  (bind _output_get (Variables|Default|SetMaxScore NewMaxScore))
  (Utilities|IsValid (Variables|/Game/Assets/Blueprints/GameMode/EndlessHUD.EndlessHUD_C|GetTouchInterfaceRef _hudref)
    (:Is%20Valid
      _)
    (:Is%20Not%20Valid
      (bind _returnvalue (UserInterface|CreateWidget "/Game/Assets/Blueprints/UI/WB_S_GameInterface.WB_S_GameInterface_C"))
      (Variables|/Game/Assets/Blueprints/GameMode/EndlessHUD.EndlessHUD_C|SetTouchInterfaceRef _hudref _returnvalue)))
  (Default|SetGoal (Variables|/Game/Assets/Blueprints/UI/WB_S_GameInterface.WB_S_GameInterface_C|GetMaxScoreWidget (Variables|/Game/Assets/Blueprints/GameMode/EndlessHUD.EndlessHUD_C|GetTouchInterfaceRef (Variables|Default|GetHUDRef))) _output_get))