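; ArcadeTrigger is a trigger actor that starts arcade play when the car enters its collision component.
; It caches the EndlessGameMode at BeginPlay.
; On overlap with a CarWithCamera component tagged "Car", and only when the game instance is not in endless mode, it passes the game mode's ArcadeState to StartArcade on the first player's EndlessPC.
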(event OnComponentBeginOverlap(CollisionComponent)
  (params (OverlappedComponent :type Primitive%20Component%20Object%20Reference) (OtherActor :type Actor%20Object%20Reference) (OtherComp :type Primitive%20Component%20Object%20Reference) (OtherBodyIndex :type Integer) (bFromSweep :type Boolean) (SweepResult :type Hit%20Result%20Structure%20%28by%20ref%29))
  (Utilities|Casting|CastToCarWithCamera OtherActor)
  (if (and (not (Variables|/Game/Assets/Blueprints/GameMode/MyGameInstance.MyGameInstance_C|GetIsEndless (.AsMy%20Game%20Instance (Utilities|Casting|CastToMyGameInstance (Game|GetGameInstance))))) (Components|ComponentHasTag OtherComp "Car"))
    (Default|StartArcade (.AsEndless%20PC (Utilities|Casting|CastToEndlessPC (Game|GetPlayerController 0))) (Variables|/Game/Assets/Blueprints/GameMode/EndlessGameMode.EndlessGameMode_C|GetArcadeState (Variables|Default|GetGMRef)))))

(event EventBeginPlay
  (Variables|Default|SetGMRef (.AsEndless%20Game%20Mode (Utilities|Casting|CastToEndlessGameMode (Game|GetGameMode)))))

(fn ConstructionScript)